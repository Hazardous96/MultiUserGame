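; Base pickup actor that reacts when the player character overlaps its collision and shows its texture on the HUD.
; A DoOnce-guarded overlap stores the character and calls Use, an empty hook presumably meant for child pickups to override.
; It then passes PickupTexture to the first BP_Hud widget found, hides the mesh and destroys itself.
; The texture name is also printed as debug output.
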(event OnComponentBeginOverlap(Collision)
  (params (OverlappedComponent :type Primitive%20Component%20Object%20Reference) (OtherActor :type Actor%20Object%20Reference) (OtherComp :type Primitive%20Component%20Object%20Reference) (OtherBodyIndex :type Integer) (bFromSweep :type Boolean) (SweepResult :type Hit%20Result%20Structure%20%28by%20ref%29))
  (bind (_asplayer_character _bsuccess) (Utilities|Casting|CastToPlayerCharacter OtherActor))
  (if _bsuccess
    (Utilities|FlowControl|DoOnce false
      (:Completed
        (Development|PrintString (Utilities|GetDisplayName (Variables|Default|GetPickupTexture)))
        (Variables|Default|SetCharacter _asplayer_character)
        (CallFunction|Use)
        (bind _foundwidgets (Widget|GetAllWidgetsOfClass "/Game/Hud/Widgets/BP_Hud.BP_Hud_C" true))
        (Default|SetPickupTexture (Utilities|Array|Get(acopy) _foundwidgets) (Variables|Default|GetPickupTexture))
        (Rendering|SetVisibility (Variables|Default|GetMesh) false false)
        (Actor|DestroyActor)))))

(event EventBeginPlay)

(event Collision|EventActorBeginOverlap
  (params (OtherActor :type Actor%20Object%20Reference)))

(event EventTick
  (params (DeltaSeconds :type Float%20%28single-precision%29)))

(fn ConstructionScript)

(fn Use)