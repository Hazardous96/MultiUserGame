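; BP_LifePickup is a pickup actor that grants an extra life to whichever player overlaps its Collision component, then destroys itself.
; The overlap event tells players apart by actor tag and increments that player's Lives.
; Player 1 is reached through an AsPlayerCharacter reference not assigned in the visible graphs, while Player 2 is taken as the first BP_Player2 found in the world.
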(event OnComponentBeginOverlap(Collision)
  (params (OverlappedComponent :type Primitive%20Component%20Object%20Reference) (OtherActor :type Actor%20Object%20Reference) (OtherComp :type Primitive%20Component%20Object%20Reference) (OtherBodyIndex :type Integer) (bFromSweep :type Boolean) (SweepResult :type Hit%20Result%20Structure%20%28by%20ref%29))
  (bind _asplayercharacter (Variables|Default|GetAsPlayerCharacter))
  (if (Actor|ActorHasTag OtherActor "Player 1")
    (bind _result (Math|Integer|IncrementInt (Variables|/Game/PlayerCharacter/PlayerCharacter.PlayerCharacter_C|GetLives _asplayercharacter))
      (:%20%20
        (Variables|/Game/PlayerCharacter/PlayerCharacter.PlayerCharacter_C|SetLives _asplayercharacter _result)
        (Actor|DestroyActor :!label _label)))
    (elif (Actor|ActorHasTag OtherActor "Player 2")
      (bind _outactors (Actor|GetAllActorsOfClass "/Game/Player2/BP_Player2.BP_Player2_C"))
      (Variables|Default|SetPlayer2 (Utilities|Array|Get(acopy) _outactors))
      (bind _result_2 (Math|Integer|IncrementInt (Variables|/Game/Player2/BP_Player2.BP_Player2_C|GetLives (Variables|Default|GetPlayer2)))
        (:%20%20
          (Variables|/Game/Player2/BP_Player2.BP_Player2_C|SetLives (Variables|Default|GetPlayer2) _result_2)
          (goto _label))))))

(event EventBeginPlay)

(event Collision|EventActorBeginOverlap
  (params (OtherActor :type Actor%20Object%20Reference)))

(event EventTick
  (params (DeltaSeconds :type Float%20%28single-precision%29)))

(fn ConstructionScript)