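; BP_DoubleDamage is a double-damage power-up that boosts ammo actors overlapping its Collision component.
; The overlapping actor's Player 1 or Player 2 tag selects a cast to BP_BasicAmmo or BP_Player2_Ammo, whose Damage is then doubled.
; After a LastingTime delay it assigns Damage to itself, so the boost is not reverted, then destroys the power-up.
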(event OnComponentBeginOverlap(Collision)
  (params (OverlappedComponent :type Primitive%20Component%20Object%20Reference) (OtherActor :type Actor%20Object%20Reference) (OtherComp :type Primitive%20Component%20Object%20Reference) (OtherBodyIndex :type Integer) (bFromSweep :type Boolean) (SweepResult :type Hit%20Result%20Structure%20%28by%20ref%29))
  (bind _lastingtime (Variables|Default|GetlastingTime))
  (if (Actor|ActorHasTag OtherActor "Player 1")
    (bind _asbp_basic_ammo (Utilities|Casting|CastToBP_BasicAmmo OtherActor))
    (Variables|/Game/PlayerCharacter/BP_BasicAmmo.BP_BasicAmmo_C|SetDamage _asbp_basic_ammo (* (Variables|/Game/PlayerCharacter/BP_BasicAmmo.BP_BasicAmmo_C|GetDamage _asbp_basic_ammo) 2.0))
    (Utilities|FlowControl|Delay _lastingtime)
    (Variables|/Game/PlayerCharacter/BP_BasicAmmo.BP_BasicAmmo_C|SetDamage _asbp_basic_ammo (Variables|/Game/PlayerCharacter/BP_BasicAmmo.BP_BasicAmmo_C|GetDamage _asbp_basic_ammo))
    (Actor|DestroyActor :!label _label)
    (elif (Actor|ActorHasTag OtherActor "Player 2")
      (bind _asbp_player_2_ammo (Utilities|Casting|CastToBP_Player2_Ammo OtherActor))
      (Variables|/Game/PlayerCharacter/BP_Player2_Ammo.BP_Player2_Ammo_C|SetDamage _asbp_player_2_ammo (* (Variables|/Game/PlayerCharacter/BP_Player2_Ammo.BP_Player2_Ammo_C|GetDamage _asbp_player_2_ammo) 2.0))
      (Utilities|FlowControl|Delay _lastingtime)
      (Variables|/Game/PlayerCharacter/BP_Player2_Ammo.BP_Player2_Ammo_C|SetDamage _asbp_player_2_ammo (Variables|/Game/PlayerCharacter/BP_Player2_Ammo.BP_Player2_Ammo_C|GetDamage _asbp_player_2_ammo))
      (goto _label))))

(event EventBeginPlay)

(event Collision|EventActorBeginOverlap
  (params (OtherActor :type Actor%20Object%20Reference)))

(event EventTick
  (params (DeltaSeconds :type Float%20%28single-precision%29)))

(fn ConstructionScript)