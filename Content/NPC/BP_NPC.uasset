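; Companion NPC that attaches to the player's NPCSocket and is meant to fire at nearby on-screen enemies.
; Looping timers mirror the player's health and scan BP_BaseEnemy actors by range, using screen projection as the visibility test.
; The line trace and randomised projectile spawn are unwired, so it never fires.
; At zero health, delayed Death destroys it, spawns a replacement at the original transform and calls attach on itself, not the replacement.
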(event Custom|Death
  ;[1 1 1] Death Event - If player is dead destroy actor respawn another at NPc scke location and attach to player
  (Actor|DestroyActor)
  (bind _asplayer_character (Utilities|Casting|CastToPlayerCharacter (Game|GetPlayerCharacter 0)))
  (Variables|Default|SetCharRef _asplayer_character)
  (Game|SpawnActorfromClass "BP_NPC_C" (Variables|Default|GetSpawnLocation) "Undefined" 0 0)
  (Transformation|AttachActorToActor (Variables|Default|GetCharRef) "NPCSocket" "KeepWorld" "KeepWorld" "KeepWorld" true)
  (Variables|Default|SetHealth (Variables|/Game/PlayerCharacter/PlayerCharacter.PlayerCharacter_C|GetHealth (Variables|Default|GetCharRef))))

(event Custom|SetHealth
  (bind _charref (Variables|Default|GetCharRef))
  ;[1 1 1] Update health variable every .5 seconds
  (if (not (Variables|Default|GetisDead))
    (Utilities|IsValid _charref
      (:Is%20Valid
        (Variables|Default|SetHealth (Variables|/Game/PlayerCharacter/PlayerCharacter.PlayerCharacter_C|GetHealth _charref))))))

(event Custom|FireAtEnemy
  ;[1 1 1] Fire At player if in range and can see (can only see if enemy is on screen)
  (bind _outactors (Actor|GetAllActorsOfClass "/Game/Enemies/BP_BaseEnemy.BP_BaseEnemy_C"))
  (bind _output_get (Variables|Default|SetAllEnemies _outactors))
  (bind (_array_element _array_index) (Utilities|Array|ForEachLoopwithBreak _output_get :!label _label)
    (:LoopBody
      (if (<= (Transformation|GetDistanceTo self _array_element) (Variables|Default|GetRange))
        (Variables|Default|SetCanSeeEnemy (CallFunction|SetCanSee _array_element))
        (goto _label Break)
        (else
          (Utilities|Array|RemoveIndex (Variables|Default|GetAllEnemies) _array_index))))))

(event EventBeginPlay
  ;[1 1 1] On spawn attach to player
  (Variables|Default|SetSpawnLocation (Transformation|GetActorTransform))
  (Transformation|AttachActorToActor (Game|GetPlayerCharacter 0) "NPCSocket" "KeepWorld" "KeepWorld" "KeepWorld" true)
  (Class|Actor|AddActorWorldRotation "0, 0, 0")
  (bind _asplayer_character (Utilities|Casting|CastToPlayerCharacter (Game|GetPlayerCharacter 0)))
  (bind _output_get (Variables|Default|SetCharRef _asplayer_character))
  (if (not (Variables|/Game/PlayerCharacter/PlayerCharacter.PlayerCharacter_C|GetisDead _output_get))
    (Utilities|Time|SetTimerbyEvent (delegate Custom|SetHealth) 0.5 true)
    (bind _returnvalue (Utilities|Time|SetTimerbyEvent (delegate Custom|FireAtEnemy) 0.3 true :!label _label))
    (if (Variables|Default|GetCanSeeEnemy)
      (Utilities|FlowControl|Delay 3.0)
      (Utilities|Time|ClearandInvalidateTimerbyHandle _returnvalue)
      (Utilities|FlowControl|Delay 3.0)
      (goto _label))))

(event EventTick
  (params (DeltaSeconds :type Float%20%28single-precision%29))
  ;[1 1 1] Test if player is dead if so wiat 5 second the run death event
  (if (<= (Variables|Default|GetHealth) 0.0)
    (Utilities|FlowControl|Delay 5.0)
    (CallFunction|Death)))

(fn ConstructionScript)

(fn SetCanSee
  (params (Enemy :type Actor%20Object%20Reference))
  (return (.ReturnValue (Class|PlayerController|ProjectWorldLocationtoScreen (Game|GetPlayerController 0) (Transformation|GetActorLocation Enemy) true))))

(fn SetProjectileSpawn
  (params (self2 :type Actor%20Object%20Reference))
  (bind _mesh (Variables|Character|GetMesh))
  (return (Math|Transform|MakeTransform (Transformation|GetSocketLocation _mesh "Muzzle") (Math|Rotator|FindLookatRotation (Transformation|GetSocketLocation _mesh "Muzzle") (Math|Random|RandomPointinBoundingBox (Transformation|GetActorLocation self2) "500.000000,500.000000,500.000000")))))

(fn GetHealth
  (return 0.0))

(fn SetCharacterRef
  (params (OtherActor :type Actor%20Object%20Reference))
  (return (Game|GetPlayerCharacter 0)))