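; Second boss actor: runs a looping random attack selector, switches phase at half health, and shows the level-complete widget on death.
; Phase 0 fires timed twin lasers or spawns toy-food obstacles; phase 1 fires twin plasma or a telegraphed beam, shots aimed by player-directed traces.
; SRV wrapper events forward attacks and damage/kill credit, branching on Player1, NPC and Player2 ammo tags.
; Tick updates the player's spawn location.
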(event Custom|SRV_NPC_Damage
  (params (damageDelt :type Float%20%28single-precision%29) (NPC :type BP%20NPC%20Object%20Reference))
  ;[1 1 1] NPC Damage + Score
  (CallFunction|NPCDamage damageDelt NPC))

(event Custom|SRV_Player2Damage
  (params (damageDelt :type Float%20%28single-precision%29) (P2 :type BP%20Player%202%20Object%20Reference))
  ;[1 1 1] Player2 Damaged + Score
  (CallFunction|Player2Damage damageDelt P2))

(event Custom|SRVActionSelector
  (CallFunction|ActionSelector))

(event Custom|SRVRightLaserShot
  ;[1 1 1] LaserShot
  (CallFunction|RightLaserShot))

(event Custom|SRVLeftLaserShot
  ;[1 1 1] LaserShot
  (CallFunction|LeftLaserShot))

(event Custom|SRVSpawnObstacle
  ;[1 1 1] SpawnObstacle
  (CallFunction|SpawnObstacle))

(event Custom|SRVLaserBeam
  ;[1 1 1] LaserBeam
  (CallFunction|LaserBeam))

(event Custom|SRV_Player2Destroy
  ;[1 1 1] Player2 Damaged + Score
  (CallFunction|Player2Destroy))

(event Custom|SRVLeftPlasmaShot
  ;[1 1 1] PlasmaShot
  (CallFunction|LeftPlasmaShot))

(event Custom|LeftPlasmaShot
  (bind _plasmashot1 (Variables|Default|GetPlasmaShot1))
  (bind _returnvalue (Transformation|GetWorldLocation _plasmashot1))
  ;[1 1 1] PlasmaShot
  (bind _outhit (Collision|LineTraceByChannel (Transformation|GetWorldLocation (Variables|Default|GetPlasmaShot1)) (+ (Transformation|GetWorldLocation (Variables|/Script/Engine.Actor|GetRootComponent (Game|GetPlayerCharacter 0))) "5000.000000,0.000000, 0") "TraceTypeQuery2" false 0 "None"))
  (if (.ReturnValue (Class|PlayerController|ProjectWorldLocationtoScreen (Game|GetPlayerController 0) (Transformation|GetActorLocation) false))
    (Game|SpawnActorfromClass "/Game/Bosses/Boss1/BP_Boss1PlasmaShot.BP_Boss1PlasmaShot_C" (Math|Transform|MakeTransform _returnvalue (Math|Rotator|FindLookatRotation _returnvalue (Math|Random|RandomPointinBoundingBox (Math|Vector|SelectVector (.ImpactPoint (Collision|BreakHitResult _outhit)) (.TraceEnd (Collision|BreakHitResult _outhit)) (.bBlockingHit (Collision|BreakHitResult _outhit))) "0.000000,500.000000,500.000000"))) "Undefined" 0 0)))

(event Custom|SRV_NPC_Destroy
  ;[1 1 1] NPC Damage + Score
  (CallFunction|NPCDestroy))

(event Custom|Dead
  ;[1 1 1] Dead
  (if (Actor|ActorHasTag "Player1_Ammo")
    (bind _asplayer_character (Utilities|Casting|CastToPlayerCharacter (Game|GetPlayerCharacter 0)))
    (bind _result (Math|Integer|IncrementInt (Variables|/Game/PlayerCharacter/PlayerCharacter.PlayerCharacter_C|GetenemiesKilled _asplayer_character))
      (:%20%20
        (Variables|/Game/PlayerCharacter/PlayerCharacter.PlayerCharacter_C|SetenemiesKilled _asplayer_character _result)))
    (elif (Actor|ActorHasTag "NPC_Ammo")
      (CallFunction|SRVNPCDestroy)
      (elif (Actor|ActorHasTag "Player2_Ammo")
        (CallFunction|SRVPlayer2Destroy)))))

(event Custom|NPC_Damage
  (params (damageDelt :type Float%20%28single-precision%29) (NPC :type BP%20NPC%20Object%20Reference))
  ;[1 1 1] NPC Damage + Score
  (Variables|/Game/NPC/BP_NPC.BP_NPC_C|SetdamageDelt NPC damageDelt))

(event Custom|NPC_Destroy
  ;[1 1 1] NPC Damage + Score
  (bind _outactors (Actor|GetAllActorsOfClass "/Game/NPC/BP_NPC.BP_NPC_C"))
  (bind _result (Math|Integer|IncrementInt (Variables|/Game/NPC/BP_NPC.BP_NPC_C|GetEnemiesKilled (Utilities|Array|Get(acopy) _outactors)))
    (:%20%20
      (Variables|/Game/NPC/BP_NPC.BP_NPC_C|SetEnemiesKilled (Utilities|Array|Get(acopy) _outactors) _result)
      (Variables|/Game/NPC/BP_NPC.BP_NPC_C|SetScore (Utilities|Array|Get(acopy) _outactors) (+ (Variables|/Game/NPC/BP_NPC.BP_NPC_C|GetScore (Utilities|Array|Get(acopy) _outactors)) (Variables|Default|GetaddScore))))))

(event Custom|LaserBeam
  (bind _bigattack (Variables|Default|GetBigAttack))
  (bind _returnvalue (Transformation|GetWorldLocation _bigattack))
  ;[1 1 1] LaserBeam
  (bind _outhit (Collision|LineTraceByChannel (Transformation|GetWorldLocation (Variables|Default|GetBigAttack)) (+ (Transformation|GetWorldLocation (Variables|/Script/Engine.Actor|GetRootComponent (Game|GetPlayerCharacter 0))) "2000.000000, 0, 0") "TraceTypeQuery2" false 0 "None"))
  (if (.ReturnValue (Class|PlayerController|ProjectWorldLocationtoScreen (Game|GetPlayerController 0) (Transformation|GetActorLocation) false))
    (Game|SpawnActorfromClass "/Game/Bosses/Boss1/BP_BossLaserWarning.BP_BossLaserWarning_C" (Math|Transform|MakeTransform _returnvalue (Math|Rotator|FindLookatRotation _returnvalue (Math|Vector|SelectVector (.ImpactPoint (Collision|BreakHitResult _outhit)) (.TraceEnd (Collision|BreakHitResult _outhit)) (.bBlockingHit (Collision|BreakHitResult _outhit))))) "Undefined" 0 0)
    (Utilities|FlowControl|Delay 1.5)
    (Game|SpawnActorfromClass "/Game/Bosses/Boss1/BP_Boss1LaserBeam.BP_Boss1LaserBeam_C" (Math|Transform|MakeTransform _returnvalue (Math|Rotator|FindLookatRotation _returnvalue (Math|Vector|SelectVector (.ImpactPoint (Collision|BreakHitResult _outhit)) (.TraceEnd (Collision|BreakHitResult _outhit)) (.bBlockingHit (Collision|BreakHitResult _outhit))))) "Undefined" 0 0)))

(event Custom|Player2_Damage
  (params (damageDelt :type Float%20%28single-precision%29) (P2 :type BP%20Player%202%20Object%20Reference))
  ;[1 1 1] Player2 Damaged + Score
  (Variables|/Game/Player2/BP_Player2.BP_Player2_C|SetdamageDelt P2 damageDelt))

(event Custom|Player2Destroy
  ;[1 1 1] Player2 Damaged + Score
  (bind _outactors (Actor|GetAllActorsOfClass "/Game/Player2/BP_Player2.BP_Player2_C"))
  (Variables|/Game/Player2/BP_Player2.BP_Player2_C|SetScore (Utilities|Array|Get(acopy) _outactors) (+ (Variables|/Game/Player2/BP_Player2.BP_Player2_C|GetScore (Utilities|Array|Get(acopy) _outactors)) (Variables|Default|GetaddScore)))
  (bind _result (Math|Integer|IncrementInt (Variables|/Game/Player2/BP_Player2.BP_Player2_C|GetenemiesKilled (Utilities|Array|Get(acopy) _outactors)))
    (:%20%20
      (Variables|/Game/Player2/BP_Player2.BP_Player2_C|SetenemiesKilled (Utilities|Array|Get(acopy) _outactors) _result))))

(event Custom|TakenDamage
  (params (Damage :type Float%20%28single-precision%29) (DamageCauser :type Actor%20Object%20Reference))
  ;[1 1 1] TakenDamage
  (if (Actor|ActorHasTag DamageCauser "Player1_Ammo")
    (bind _asplayer_character (Utilities|Casting|CastToPlayerCharacter (Game|GetPlayerCharacter 0)))
    (Variables|/Game/PlayerCharacter/PlayerCharacter.PlayerCharacter_C|SetdamageDelt _asplayer_character (+ (Variables|/Game/PlayerCharacter/PlayerCharacter.PlayerCharacter_C|GetdamageDelt _asplayer_character) Damage))
    (elif (Actor|ActorHasTag DamageCauser "NPC_Ammo")
      (bind _outactors (Actor|GetAllActorsOfClass "/Game/NPC/BP_NPC.BP_NPC_C"))
      (CallFunction|SRVNPCDamage (Variables|/Game/NPC/BP_NPC.BP_NPC_C|GetdamageDelt (Utilities|Array|Get(acopy) _outactors)) (Utilities|Array|Get(acopy) _outactors))
      (elif (Actor|ActorHasTag DamageCauser "Player2_Ammo")
        (bind _outactors_2 (Actor|GetAllActorsOfClass "/Game/Player2/BP_Player2.BP_Player2_C"))
        (CallFunction|SRVPlayer2Damage (Variables|/Game/Player2/BP_Player2.BP_Player2_C|GetdamageDelt (Utilities|Array|Get(acopy) _outactors_2)) (Utilities|Array|Get(acopy) _outactors_2))))))

(event Custom|SRV_TakenDamage
  (params (Damage :type Float%20%28single-precision%29) (DamageCauser :type Actor%20Object%20Reference))
  ;[1 1 1] TakenDamage
  (CallFunction|TakenDamage Damage DamageCauser))

(event Custom|LeftLaserShot
  (bind _returnvalue (Math|Random|RandomInteger 1))
  (bind _lasershot1 (Variables|Default|GetLaserShot1))
  (bind _returnvalue_2 (Transformation|GetWorldLocation _lasershot1))
  (bind _returnvalue_3 (Game|GetPlayerCharacter _returnvalue))
  ;[1 1 1] LaserShot
  (Utilities|IsValid _returnvalue_3
    (:Is%20Valid
      (bind _outhit (Collision|LineTraceByChannel (Transformation|GetWorldLocation (Variables|Default|GetLaserShot1)) (+ (Transformation|GetWorldLocation (Variables|/Script/Engine.Actor|GetRootComponent _returnvalue_3)) "5000.000000,0.000000, 0") "TraceTypeQuery2" false 0 "None"))
      (if (.ReturnValue (Class|PlayerController|ProjectWorldLocationtoScreen (Game|GetPlayerController 0) (Transformation|GetActorLocation) false))
        (Game|SpawnActorfromClass "/Game/Bosses/Boss1/BP_Boss1LaserShot.BP_Boss1LaserShot_C" (Math|Transform|MakeTransform _returnvalue_2 (Math|Rotator|FindLookatRotation _returnvalue_2 (Math|Random|RandomPointinBoundingBox (Math|Vector|SelectVector (.ImpactPoint (Collision|BreakHitResult _outhit)) (.TraceEnd (Collision|BreakHitResult _outhit)) (.bBlockingHit (Collision|BreakHitResult _outhit))) "0.000000,500.000000,500.000000"))) "Undefined" 0 0)))))

(event Custom|SRVRightPlasmaShot
  ;[1 1 1] PlasmaShot
  (CallFunction|RightPlasmaShot))

(event Custom|ActionSelector
  (bind _returnvalue (Math|Random|RandomIntegerinRange 0 2))
  (if (== (Variables|Default|GetPhase) 0) :!label _label
    (switch int _returnvalue
      (:0
        _)
      (:1
        _)
      (:2
        (CallFunction|SRVSpawnObstacle)
        (Utilities|FlowControl|Delay 1.0)
        (CallFunction|SRVSpawnObstacle)
        (Utilities|FlowControl|Delay 3.0)
        (goto _label)))
    (bind _returnvalue_2 (Utilities|Time|SetTimerbyEvent (delegate Custom|SRVRightLaserShot) 0.2 true))
    (bind _returnvalue_3 (Utilities|Time|SetTimerbyEvent (delegate Custom|SRVLeftLaserShot) 0.2 true))
    (Utilities|FlowControl|Delay 3.0)
    (Utilities|Time|PauseTimerbyHandle _returnvalue_2)
    (Utilities|Time|PauseTimerbyHandle _returnvalue_3)
    (Utilities|FlowControl|Delay 2.5)
    (goto _label)
    (else
      (switch int _returnvalue
        (:0
          _)
        (:1
          _)
        (:2
          (CallFunction|SRVLaserBeam)
          (Utilities|FlowControl|Delay 5.0)
          (goto _label)))
      (bind _returnvalue_4 (Utilities|Time|SetTimerbyEvent (delegate Custom|SRVLeftPlasmaShot) 0.15 true))
      (bind _returnvalue_5 (Utilities|Time|SetTimerbyEvent (delegate Custom|SRVRightPlasmaShot) 0.15 true))
      (Utilities|FlowControl|Delay 5.0)
      (Utilities|Time|PauseTimerbyHandle _returnvalue_4)
      (Utilities|Time|PauseTimerbyHandle _returnvalue_5)
      (Utilities|FlowControl|Delay 2.5)
      (goto _label))))

(event Custom|RightPlasmaShot
  (bind _plasmashot2 (Variables|Default|GetPlasmaShot2))
  (bind _returnvalue (Transformation|GetWorldLocation _plasmashot2))
  ;[1 1 1] PlasmaShot
  (bind _outhit (Collision|LineTraceByChannel (Transformation|GetWorldLocation (Variables|Default|GetPlasmaShot2)) (+ (Transformation|GetWorldLocation (Variables|/Script/Engine.Actor|GetRootComponent (Game|GetPlayerCharacter 0))) "5000.000000, 0, 0") "TraceTypeQuery2" false 0 "None"))
  (if (.ReturnValue (Class|PlayerController|ProjectWorldLocationtoScreen (Game|GetPlayerController 0) (Transformation|GetActorLocation) false))
    (Game|SpawnActorfromClass "/Game/Bosses/Boss1/BP_Boss1PlasmaShot.BP_Boss1PlasmaShot_C" (Math|Transform|MakeTransform _returnvalue (Math|Rotator|FindLookatRotation _returnvalue (Math|Random|RandomPointinBoundingBox (Math|Vector|SelectVector (.ImpactPoint (Collision|BreakHitResult _outhit)) (.TraceEnd (Collision|BreakHitResult _outhit)) (.bBlockingHit (Collision|BreakHitResult _outhit))) "0.000000,500.000000,500.000000"))) "Undefined" 0 0)))

(event Custom|SpawnObstacle
  ;[1 1 1] SpawnObstacle
  (Utilities|FlowControl|Delay 1.0)
  (Utilities|FlowControl|Sequence
    (:then_0
      (Game|SpawnActorfromClass "/Game/LevelItems/BP_ToyFood01.BP_ToyFood01_C" (Math|Transform|MakeTransform (Math|Random|RandomPointinBoundingBox (Transformation|GetWorldLocation (Variables|Default|GetObstacleLeft)) "0.000000,5000.000000,500.000000") "0, 0, 0" "1,1,1") "Undefined" 0 0))
    (:then_1
      (Game|SpawnActorfromClass "/Game/LevelItems/BP_ToyFood02.BP_ToyFood02_C" (Math|Transform|MakeTransform (Math|Random|RandomPointinBoundingBox (Transformation|GetWorldLocation (Variables|Default|GetObstacleCenter)) "0.000000,5000.000000,500.000000") "0, 0, 0" "1,1,1") "Undefined" 0 0))
    (:then_2
      (Game|SpawnActorfromClass "/Game/LevelItems/BP_ToyFood03.BP_ToyFood03_C" (Math|Transform|MakeTransform (Math|Random|RandomPointinBoundingBox (Transformation|GetWorldLocation (Variables|Default|GetObstacleRight)) "0.000000,5000.000000,500.000000") "0, 0, 0" "1,1,1") "Undefined" 0 0))))

(event Custom|RightLaserShot
  (bind _returnvalue (Math|Random|RandomInteger 1))
  (bind _lasershot2 (Variables|Default|GetLaserShot2))
  (bind _returnvalue_2 (Transformation|GetWorldLocation _lasershot2))
  (bind _returnvalue_3 (Game|GetPlayerCharacter _returnvalue))
  ;[1 1 1] LaserShot
  (Utilities|IsValid _returnvalue_3
    (:Is%20Valid
      (bind _outhit (Collision|LineTraceByChannel (Transformation|GetWorldLocation (Variables|Default|GetLaserShot2)) (+ (Transformation|GetWorldLocation (Variables|/Script/Engine.Actor|GetRootComponent _returnvalue_3)) "5000.000000, 0, 0") "TraceTypeQuery2" false 0 "None"))
      (if (.ReturnValue (Class|PlayerController|ProjectWorldLocationtoScreen (Game|GetPlayerController 0) (Transformation|GetActorLocation) false))
        (Game|SpawnActorfromClass "/Game/Bosses/Boss1/BP_Boss1LaserShot.BP_Boss1LaserShot_C" (Math|Transform|MakeTransform _returnvalue_2 (Math|Rotator|FindLookatRotation _returnvalue_2 (Math|Random|RandomPointinBoundingBox (Math|Vector|SelectVector (.ImpactPoint (Collision|BreakHitResult _outhit)) (.TraceEnd (Collision|BreakHitResult _outhit)) (.bBlockingHit (Collision|BreakHitResult _outhit))) "0.000000,500.000000,500.000000"))) "Undefined" 0 0)))))

(event Custom|SRV_Dead
  ;[1 1 1] Dead
  (CallFunction|Dead))

(event Game|Damage|EventAnyDamage
  (params (Damage :type Float%20%28single-precision%29) (DamageType :type Damage%20Type%20Object%20Reference) (InstigatedBy :type Controller%20Object%20Reference) (DamageCauser :type Actor%20Object%20Reference))
  ;[1 1 1] Take Damage
  (CallFunction|SRVTakenDamage Damage DamageCauser)
  (bind _output_get (Variables|Default|SetHealth (- (Variables|Default|GetHealth) Damage)))
  (Development|PrintString (Utilities|String|ToString(Float) _output_get) true true "(R=1.000000,G=0.007892,B=0.000000,A=1.000000)")
  (if (<= _output_get (Variables|Default|GetPhase_Change))
    (Variables|Default|SetPhase 1)
    (if (<= (Variables|Default|GetHealth) 0.0)
      (CallFunction|SRVDead)
      (Actor|DestroyActor)
      (bind _returnvalue (UserInterface|CreateWidget "/Game/Hud/Widgets/BP_LevelComplete.BP_LevelComplete_C"))
      (UserInterface|Viewport|AddtoViewport _returnvalue 0))
    (else
      (Variables|Default|SetPhase 0))))

(event EventTick
  (params (DeltaSeconds :type Float%20%28single-precision%29))
  (|CallParentFunction DeltaSeconds)
  (bind _asplayer_character (Utilities|Casting|CastToPlayerCharacter (Game|GetPlayerCharacter 0)))
  (Variables|/Game/PlayerCharacter/PlayerCharacter.PlayerCharacter_C|SetSpawnLocation _asplayer_character (Math|Transform|MakeTransform (.location (Transformation|GetWorldTransform (Variables|Default|GetPlayerSpawn))) "0, 0, 0" "1,1,1")))

(event EventBeginPlay
  (Variables|Default|SetPhase 0)
  (Variables|Default|SetHealth 1e+03)
  (Variables|Default|SetPhase_Change 5e+02)
  (CallFunction|SRVActionSelector))

(fn ConstructionScript
  (|CallParentFunction))