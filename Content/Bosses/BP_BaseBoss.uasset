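; BP_BaseBoss is a base boss Blueprint that moves constantly, tracks health and switches between two phases.
; Tick feeds movement input opposite its forward vector every frame.
; FindPlayer traces from the Spawn component to a random point in a flat YZ box around the player, drawing debug lines without using the hit.
; AnyDamage subtracts health and selects the second phase once health reaches the PhaseChange threshold.
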(event Custom|FindPlayer
  (Variables|Default|SetTarget (Math|Random|RandomPointinBoundingBox (Transformation|GetActorLocation (Game|GetPlayerCharacter 0)) "0.000000,1250.000000,750.000000"))
  (Collision|LineTraceByChannel (Transformation|GetWorldLocation (Variables|Default|GetSpawn)) (Variables|Default|GetTarget) "TraceTypeQuery1" false 0 "ForDuration"))

(event EventTick
  (params (DeltaSeconds :type Float%20%28single-precision%29))
  (Pawn|Input|AddMovementInput (Transformation|GetActorForwardVector) -5e+02 false))

(event Game|Damage|EventAnyDamage
  (params (Damage :type Float%20%28single-precision%29) (DamageType :type Damage%20Type%20Object%20Reference) (InstigatedBy :type Controller%20Object%20Reference) (DamageCauser :type Actor%20Object%20Reference))
  (bind _output_get (Variables|Default|SetHealth (- (Variables|Default|GetHealth) Damage)))
  (if (<= _output_get (Variables|Default|GetPhase_Change))
    (Variables|Default|SetPhase 1)
    (else
      (Variables|Default|SetPhase 0))))

(fn ConstructionScript)