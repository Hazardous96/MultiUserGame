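; BP_BaseBattery is a collectible battery pickup that restores health to either of two players.
; When its collision is overlapped, it checks for the "Player 1" or "Player 2" tag, resolving Player 2 as the first BP_Player2 in the level.
; It raises Health by the HealthGain fraction of current health, so lower health recovers less, caps it at 100, then destroys itself.
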(event OnComponentBeginOverlap(Collision)
  (params (OverlappedComponent :type Primitive%20Component%20Object%20Reference) (OtherActor :type Actor%20Object%20Reference) (OtherComp :type Primitive%20Component%20Object%20Reference) (OtherBodyIndex :type Integer) (bFromSweep :type Boolean) (SweepResult :type Hit%20Result%20Structure%20%28by%20ref%29))
  (bind _asplayercharacter (Variables|Default|GetAsPlayerCharacter))
  (if (Actor|ActorHasTag OtherActor "Player 1")
    (if (> (+ (Variables|/Game/PlayerCharacter/PlayerCharacter.PlayerCharacter_C|GetHealth _asplayercharacter) (* (Variables|/Game/PlayerCharacter/PlayerCharacter.PlayerCharacter_C|GetHealth _asplayercharacter) (Variables|Default|GethealthGain))) 1e+02)
      (Variables|/Game/PlayerCharacter/PlayerCharacter.PlayerCharacter_C|SetHealth _asplayercharacter 1e+02)
      (else
        (Variables|/Game/PlayerCharacter/PlayerCharacter.PlayerCharacter_C|SetHealth _asplayercharacter (+ (Variables|/Game/PlayerCharacter/PlayerCharacter.PlayerCharacter_C|GetHealth _asplayercharacter) (* (Variables|/Game/PlayerCharacter/PlayerCharacter.PlayerCharacter_C|GetHealth _asplayercharacter) (Variables|Default|GethealthGain))))))
    (Actor|DestroyActor :!label _label)
    (elif (Actor|ActorHasTag OtherActor "Player 2")
      (bind _outactors (Actor|GetAllActorsOfClass "/Game/Player2/BP_Player2.BP_Player2_C"))
      (Variables|Default|SetPlayer2 (Utilities|Array|Get(acopy) _outactors))
      (if (> (+ (Variables|/Game/Player2/BP_Player2.BP_Player2_C|GetHealth (Variables|Default|GetPlayer2)) (* (Variables|/Game/Player2/BP_Player2.BP_Player2_C|GetHealth (Variables|Default|GetPlayer2)) (Variables|Default|GethealthGain))) 1e+02)
        (Variables|/Game/Player2/BP_Player2.BP_Player2_C|SetHealth (Variables|Default|GetPlayer2) 1e+02)
        (goto _label)
        (else
          (Variables|/Game/Player2/BP_Player2.BP_Player2_C|SetHealth (Variables|Default|GetPlayer2) (+ (Variables|/Game/Player2/BP_Player2.BP_Player2_C|GetHealth (Variables|Default|GetPlayer2)) (* (Variables|/Game/Player2/BP_Player2.BP_Player2_C|GetHealth (Variables|Default|GetPlayer2)) (Variables|Default|GethealthGain))))
          (goto _label))))))

(event EventBeginPlay)

(event Collision|EventActorBeginOverlap
  (params (OtherActor :type Actor%20Object%20Reference)))

(event EventTick
  (params (DeltaSeconds :type Float%20%28single-precision%29)))

(fn ConstructionScript)