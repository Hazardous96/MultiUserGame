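; BP_BaseCollectable is a collectible pickup base that shows its texture as the active pickup on the HUD of a two-player game.
; On actor overlap it looks up the first top-level BP_Hud widget and calls UpdateActivePickup, using the Player1 or Player2 tag to choose the player.
; It neither destroys itself nor applies any gameplay effect.
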(event EventBeginPlay)

(event Collision|EventActorBeginOverlap
  (params (OtherActor :type Actor%20Object%20Reference))
  (bind _foundwidgets (Widget|GetAllWidgetsOfClass "/Game/Hud/Widgets/BP_Hud.BP_Hud_C" true))
  (Variables|Default|SetHUD (Utilities|Array|Get(acopy) _foundwidgets))
  (if (Actor|ActorHasTag OtherActor "Player1")
    (Default|UpdateActivePickup (Variables|Default|GetHUD) (Variables|Default|Gettexture) true)
    (elif (Actor|ActorHasTag OtherActor "Player2")
      (Default|UpdateActivePickup (Variables|Default|GetHUD) (Variables|Default|Gettexture) false))))

(event EventTick
  (params (DeltaSeconds :type Float%20%28single-precision%29)))

(fn ConstructionScript)