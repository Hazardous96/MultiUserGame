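; Shield pickup collectible that sets an overlapping player's Shield to full and shows its texture as that player's active pickup.
; BeginPlay caches the BP_Hud widget, and the collision overlap uses Player1/Player2 actor tags to choose the player.
; The shield goes to the first PlayerCharacter or BP_Player2 found by class lookup, not to the overlapping actor.
; Only the Player1 branch destroys the pickup.
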(event OnComponentBeginOverlap(Collision)
  (params (OverlappedComponent :type Primitive%20Component%20Object%20Reference) (OtherActor :type Actor%20Object%20Reference) (OtherComp :type Primitive%20Component%20Object%20Reference) (OtherBodyIndex :type Integer) (bFromSweep :type Boolean) (SweepResult :type Hit%20Result%20Structure%20%28by%20ref%29))
  (if (Actor|ActorHasTag OtherActor "Player1")
    (bind _returnvalue (Actor|GetActorOfClass "/Game/PlayerCharacter/PlayerCharacter.PlayerCharacter_C"))
    (Variables|/Game/PlayerCharacter/PlayerCharacter.PlayerCharacter_C|SetShield _returnvalue 1e+02)
    (Default|UpdateActivePickup (Variables|Default|GetHUD) (Variables|Default|Gettexture) true)
    (Actor|DestroyActor)
    (elif (Actor|ActorHasTag OtherActor "Player2")
      (bind _outactors (Actor|GetAllActorsOfClass "/Game/Player2/BP_Player2.BP_Player2_C"))
      (Variables|Default|SetPlayer2 (Utilities|Array|Get(acopy) _outactors))
      (Variables|/Game/Player2/BP_Player2.BP_Player2_C|SetShield (Variables|Default|GetPlayer2) 1e+02)
      (Default|UpdateActivePickup (Variables|Default|GetHUD) (Variables|Default|Gettexture) false))))

(event Collision|EventActorBeginOverlap
  (params (OtherActor :type Actor%20Object%20Reference))
  (|CallParentFunction OtherActor) ; This node is disabled and will not be called.\nDrag off pins to build functionality.
)

(event EventTick
  (params (DeltaSeconds :type Float%20%28single-precision%29))
  (|CallParentFunction DeltaSeconds) ; This node is disabled and will not be called.\nDrag off pins to build functionality.
)

(event EventBeginPlay
  (bind _foundwidgets (Widget|GetAllWidgetsOfClass "/Game/Hud/Widgets/BP_Hud.BP_Hud_C" true))
  (Variables|Default|SetHUD (Utilities|Array|Get(acopy) _foundwidgets)))

(fn ConstructionScript
  (|CallParentFunction))