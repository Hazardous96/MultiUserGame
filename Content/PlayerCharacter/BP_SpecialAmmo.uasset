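; BP_SpecialAmmo is a player special-ammo projectile that homes in on an enemy and carries high damage.
; On BeginPlay it targets the mesh of the first BP_BaseEnemy found, sets damage and a short lifespan, and briefly delays enabling sphere collision.
; A looping timer then reassigns homing to the first remaining enemy whenever the current target becomes invalid.
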(event Custom|NewEnemy
  ;[1 1 1] Retarget Enemy
  (Utilities|IsValid (Variables|Default|GetEnemy)
    (:Is%20Not%20Valid
      (bind _outactors (Actor|GetAllActorsOfClass "/Game/Enemies/BP_BaseEnemy.BP_BaseEnemy_C"))
      (bind _output_get (Variables|Default|SetEnemy (Utilities|Array|Get(acopy) _outactors)))
      (Variables|/Script/Engine.ProjectileMovementComponent|SetHomingTargetComponent (Variables|Default|GetProjectileMovement) (Variables|/Script/Engine.Character|GetMesh _output_get)))))

(event EventBeginPlay
  (|CallParentFunction)
  (Collision|SetCollisionEnabled (Variables|Default|GetSphere) "NoCollision")
  ;[1 1 1] Target Enemy
  (bind _outactors (Actor|GetAllActorsOfClass "/Game/Enemies/BP_BaseEnemy.BP_BaseEnemy_C"))
  (bind _output_get (Variables|Default|SetEnemy (Utilities|Array|Get(acopy) _outactors)))
  (Variables|/Script/Engine.ProjectileMovementComponent|SetHomingTargetComponent (Variables|Default|GetProjectileMovement) (Variables|/Script/Engine.Character|GetMesh _output_get))
  (Variables|Default|SetDamage 5e+02)
  (Actor|SetLifeSpan 5.0)
  (Utilities|FlowControl|Delay 0.2)
  (Collision|SetCollisionEnabled (Variables|Default|GetSphere) "QueryAndPhysics")
  (Utilities|Time|SetTimerbyEvent (delegate Custom|NewEnemy) 0.5 true))

(fn ConstructionScript
  (|CallParentFunction))