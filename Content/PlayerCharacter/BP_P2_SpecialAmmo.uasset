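; BP_P2_SpecialAmmo is a high-damage homing projectile that seeks enemies, named as Player 2's special ammo.
; On spawn it homes on the BP_BaseEnemy closest to player character 0, with a five-second lifespan.
; Sphere collision stays disabled briefly after spawn.
; A looping timer retargets to the first enemy found, not the closest, whenever the current target becomes invalid.
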(event Custom|NewEnemy
  ;[1 1 1] Retarget Enemy
  (Utilities|IsValid (Variables|Default|GetEnemy)
    (:Is%20Not%20Valid
      (bind _outactors (Actor|GetAllActorsOfClass "/Game/Enemies/BP_BaseEnemy.BP_BaseEnemy_C"))
      (bind _output_get (Variables|Default|SetEnemy (Utilities|Array|Get(acopy) _outactors)))
      (Variables|/Script/Engine.ProjectileMovementComponent|SetHomingTargetComponent (Variables|Default|GetProjectileMovement) (Variables|/Script/Engine.Character|GetMesh _output_get)))))

(event EventBeginPlay
  (bind _returnvalue (Game|GetPlayerCharacter 0))
  ;[1 1 1] Target Enemy
  (|CallParentFunction)
  (Collision|SetCollisionEnabled (Variables|Default|GetSphere) "NoCollision")
  ;;[1 1 1] GetClosestEnemy
  (bind _outactors (Actor|GetAllActorsOfClass "/Game/Enemies/BP_BaseEnemy.BP_BaseEnemy_C"))
  (Variables|Default|SetDistance (Transformation|GetDistanceTo _returnvalue (Utilities|Array|Get(acopy) _outactors)))
  (for (_array_element _array_index) _outactors
    (if (< (Transformation|GetDistanceTo _returnvalue _array_element) (Variables|Default|GetDistance))
      (Variables|Default|SetDistance (Transformation|GetDistanceTo _returnvalue _array_element))
      (bind _output_get (Variables|Default|SetClosestEnemy _array_index))))
  (bind _output_get_2 (Variables|Default|SetEnemy (Utilities|Array|Get(acopy) _outactors _output_get)))
  (Variables|/Script/Engine.ProjectileMovementComponent|SetHomingTargetComponent (Variables|Default|GetProjectileMovement) (Variables|/Script/Engine.Character|GetMesh _output_get_2))
  (Variables|Default|SetDamage 5e+02)
  (Actor|SetLifeSpan 5.0)
  (Utilities|FlowControl|Delay 0.2)
  (Collision|SetCollisionEnabled (Variables|Default|GetSphere) "QueryAndPhysics")
  (Utilities|Time|SetTimerbyEvent (delegate Custom|NewEnemy) 0.5 true))

(fn ConstructionScript
  (|CallParentFunction))