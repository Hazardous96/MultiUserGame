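; BP_BasicAmmo is a short-lived projectile in the PlayerCharacter folder that explodes and deals damage on impact.
; A sphere component hit on a valid actor passes a filter comparing a Turret_Projectile inequality check against the Player tag, normally excluding both.
; A passing hit spawns an explosion emitter at the impact point, applies damage and destroys the projectile.
; BeginPlay sets a brief life span so stray shots expire.
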(event OnComponentHit(Sphere)
  (params (HitComponent :type Primitive%20Component%20Object%20Reference) (OtherActor :type Actor%20Object%20Reference) (OtherComp :type Primitive%20Component%20Object%20Reference) (NormalImpulse :type Vector :default "0, 0, 0") (Hit :type Hit%20Result%20Structure%20%28by%20ref%29))
  ;[1 1 1] Destroyed
  (Utilities|IsValid OtherActor
    (:Is%20Valid
      (if (Math|Boolean|NotEqual(Boolean) (!= OtherActor "/Game/Enemies/TurretEnemy/Turret_Projectile.Turret_Projectile") (Actor|ActorHasTag OtherActor "Player"))
        (Effects|SpawnEmitteratLocation "/Game/StarterContent/Particles/P_Explosion.P_Explosion" (.impactpoint Hit))
        (Game|Damage|ApplyDamage OtherActor (Variables|Default|GetDamage) 0 self)
        (Actor|DestroyActor)))))

(event EventBeginPlay
  ;[1 1 1] Destroyed
  (Actor|SetLifeSpan 2.0))

(fn ConstructionScript)