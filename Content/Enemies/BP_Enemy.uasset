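; BP_Enemy is an enemy with health, a movement speed and a death flag.
; On BeginPlay, binding the damage handler and copying Speed to FloatingPawnMovement's max speed both sit behind a BP_EnemySpawner cast with no object wired in.
; The damage handler subtracts damage from Health and sets IsDead once it is depleted; nothing in this graph acts on that flag.
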(event Custom|Damaged
  (params (DamagedActor :type Actor%20Object%20Reference) (Damage :type Float%20%28single-precision%29) (DamageType :type Damage%20Type%20Object%20Reference) (InstigatedBy :type Controller%20Object%20Reference) (DamageCauser :type Actor%20Object%20Reference))
  ;[1 1 1] Damaged/Die
  (bind _output_get (Variables|Default|SetHealth (- (Variables|Default|GetHealth) Damage)))
  (if (<= _output_get 0.0)
    (Variables|Default|SetisDead true)))

(event EventBeginPlay
  (Utilities|Casting|CastToBP_EnemySpawner)
  (EventDispatchers|AssignOnTakeAnyDamage (delegate Custom|Damaged))
  (Variables|/Script/Engine.FloatingPawnMovement|SetMaxSpeed (Variables|Default|GetFloatingPawnMovement) (Variables|Default|GetSpeed)))

(event Collision|EventActorBeginOverlap
  (params (OtherActor :type Actor%20Object%20Reference)))

(event EventTick
  (params (DeltaSeconds :type Float%20%28single-precision%29)))

(fn ConstructionScript)