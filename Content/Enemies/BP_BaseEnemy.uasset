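; Base enemy actor that deals damage to a player character on hit, then destroys itself.
; AnyDamage uses the causer's ammo tag to credit Player 1, Player 2 or the NPC with damage dealt.
; Death spawns an explosion and adds score to the killer, with kill counts only for Player 1 and the NPC.
; Player 2 reference and line-of-sight logic exist, but their calls are unwired.
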(event Custom|NPC_Damaged
  (params (damageDelt :type Float%20%28single-precision%29) (NPC :type BP%20NPC%20Object%20Reference))
  ;[1 1 1] NPC Damaged
  (if (> (stale Game|Damage|EventAnyDamage Damage) (Variables|Default|GetHealth))
    (Variables|/Game/NPC/BP_NPC.BP_NPC_C|SetdamageDelt NPC (+ (Variables|Default|GetHealth) damageDelt))
    (Variables|Default|SetHealth 0.0)
    (else
      (Variables|Default|SetHealth (- (Variables|Default|GetHealth) (stale Game|Damage|EventAnyDamage Damage)))
      (Variables|/Game/NPC/BP_NPC.BP_NPC_C|SetdamageDelt NPC (+ (stale Game|Damage|EventAnyDamage Damage) damageDelt))))
  (if (<= (Variables|Default|GetHealth) 0.0)
    (Effects|SpawnEmitteratLocation "/Game/StarterContent/Particles/P_Explosion.P_Explosion" (Transformation|GetActorLocation) "0, 0, 0" "10.000000,10.000000,10.000000")
    (Actor|DestroyActor)
    (Variables|Default|SetisDead true)
    (bind _outactors (Actor|GetAllActorsOfClass "/Game/NPC/BP_NPC.BP_NPC_C"))
    (bind _result (Math|Integer|IncrementInt (Variables|/Game/NPC/BP_NPC.BP_NPC_C|GetEnemiesKilled (Utilities|Array|Get(acopy) _outactors)))
      (:%20%20
        (Variables|/Game/NPC/BP_NPC.BP_NPC_C|SetEnemiesKilled (Utilities|Array|Get(acopy) _outactors) _result)
        (Variables|/Game/NPC/BP_NPC.BP_NPC_C|SetScore (Utilities|Array|Get(acopy) _outactors) (+ (Variables|/Game/NPC/BP_NPC.BP_NPC_C|GetScore (Utilities|Array|Get(acopy) _outactors)) (Variables|Default|GetaddScore)))))))

(event Custom|Player2_Damage
  (params (damageDelt :type Float%20%28single-precision%29) (P2 :type BP%20Player%202%20Object%20Reference))
  ;[1 1 1] Player Damaged
  (if (> (stale Game|Damage|EventAnyDamage Damage) (Variables|Default|GetHealth))
    (Variables|/Game/Player2/BP_Player2.BP_Player2_C|SetdamageDelt P2 (+ (Variables|Default|GetHealth) damageDelt))
    (Variables|Default|SetHealth 0.0)
    (else
      (Variables|Default|SetHealth (- (Variables|Default|GetHealth) (stale Game|Damage|EventAnyDamage Damage)))
      (Variables|/Game/Player2/BP_Player2.BP_Player2_C|SetdamageDelt P2 (+ (stale Game|Damage|EventAnyDamage Damage) damageDelt))))
  (if (<= (Variables|Default|GetHealth) 0.0)
    (Effects|SpawnEmitteratLocation "/Game/StarterContent/Particles/P_Explosion.P_Explosion" (Transformation|GetActorLocation) "0, 0, 0" "10.000000,10.000000,10.000000")
    (Actor|DestroyActor)
    (Variables|Default|SetisDead true)
    (bind _outactors (Actor|GetAllActorsOfClass "/Game/Player2/BP_Player2.BP_Player2_C"))
    (Variables|/Game/Player2/BP_Player2.BP_Player2_C|SetScore (Utilities|Array|Get(acopy) _outactors) (+ (Variables|/Game/Player2/BP_Player2.BP_Player2_C|GetScore (Utilities|Array|Get(acopy) _outactors)) (Variables|Default|GetaddScore)))))

(event Custom|GetPlayer2Ref
  (bind _asbp_player_2 (Utilities|Casting|CastToBP_Player2 (Game|GetPlayerCharacter 0)))
  (Variables|Default|SetPlayer2Ref _asbp_player_2))

(event Custom|SetCanSee
  (Variables|Default|SetCanSeeP1 (Controller|LineOfSightTo (Game|GetPlayerController 0) (Variables|Default|GetPlayerRef) "0, 0, 0" false))
  (Variables|Default|SetCanSeeP2 (Controller|LineOfSightTo (Game|GetPlayerController 1) (Variables|Default|GetPlayer2Ref) "0, 0, 0" false)))

(event Collision|EventHit
  (params (MyComp :type Primitive%20Component%20Object%20Reference) (Other :type Actor%20Object%20Reference) (OtherComp :type Primitive%20Component%20Object%20Reference) (bSelfMoved :type Boolean) (HitLocation :type Vector :default "0, 0, 0") (HitNormal :type Vector :default "0, 0, 0") (NormalImpulse :type Vector :default "0, 0, 0") (Hit :type Hit%20Result%20Structure%20%28by%20ref%29))
  ;[1 1 1] Hit Damaged
  (bind _asplayer_character (Utilities|Casting|CastToPlayerCharacter Other))
  (Game|Damage|ApplyDamage _asplayer_character 2e+01 0 0)
  (Actor|DestroyActor))

(event EventBeginPlay
  ;[1 1 1] Begin Play
  (bind _asplayer_character (Utilities|Casting|CastToPlayerCharacter (Game|GetPlayerCharacter 0)))
  (Variables|Default|SetPlayerRef _asplayer_character))

(event Game|Damage|EventAnyDamage
  (params (Damage :type Float%20%28single-precision%29) (DamageType :type Damage%20Type%20Object%20Reference) (InstigatedBy :type Controller%20Object%20Reference) (DamageCauser :type Actor%20Object%20Reference))
  ;[1 1 1] TakenDamage
  (if (Actor|ActorHasTag DamageCauser "Player1_Ammo")
    (bind _asplayer_character (Utilities|Casting|CastToPlayerCharacter (Game|GetPlayerCharacter 0)))
    ;;[1 1 1] Player Damaged
    (if (> Damage (Variables|Default|GetHealth))
      (Variables|/Game/PlayerCharacter/PlayerCharacter.PlayerCharacter_C|SetdamageDelt _asplayer_character (+ (Variables|Default|GetHealth) (Variables|/Game/PlayerCharacter/PlayerCharacter.PlayerCharacter_C|GetdamageDelt _asplayer_character)))
      (Variables|Default|SetHealth 0.0)
      (else
        (Variables|Default|SetHealth (- (Variables|Default|GetHealth) Damage))
        (Variables|/Game/PlayerCharacter/PlayerCharacter.PlayerCharacter_C|SetdamageDelt _asplayer_character (+ Damage (Variables|/Game/PlayerCharacter/PlayerCharacter.PlayerCharacter_C|GetdamageDelt _asplayer_character)))))
    (if (<= (Variables|Default|GetHealth) 0.0)
      (Effects|SpawnEmitteratLocation "/Game/StarterContent/Particles/P_Explosion.P_Explosion" (Transformation|GetActorLocation) "0, 0, 0" "10.000000,10.000000,10.000000")
      (Actor|DestroyActor)
      (Variables|Default|SetisDead true)
      (bind _asplayer_character_2 (Utilities|Casting|CastToPlayerCharacter (Game|GetPlayerCharacter 0)))
      (Variables|/Game/PlayerCharacter/PlayerCharacter.PlayerCharacter_C|SetScore _asplayer_character_2 (+ (Variables|/Game/PlayerCharacter/PlayerCharacter.PlayerCharacter_C|GetScore _asplayer_character_2) (Variables|Default|GetaddScore)))
      (bind _result (Math|Integer|IncrementInt (Variables|/Game/PlayerCharacter/PlayerCharacter.PlayerCharacter_C|GetenemiesKilled _asplayer_character_2))
        (:%20%20
          (Variables|/Game/PlayerCharacter/PlayerCharacter.PlayerCharacter_C|SetenemiesKilled _asplayer_character_2 _result)
          (Development|PrintString "bullet"))))
    (elif (Actor|ActorHasTag DamageCauser "NPC_Ammo")
      (bind _outactors (Actor|GetAllActorsOfClass "/Game/NPC/BP_NPC.BP_NPC_C"))
      (CallFunction|NPCDamaged (Variables|/Game/NPC/BP_NPC.BP_NPC_C|GetdamageDelt (Utilities|Array|Get(acopy) _outactors)) (Utilities|Array|Get(acopy) _outactors))
      (else
        ;[1 1 1] Player Damaged
        (if (Actor|ActorHasTag DamageCauser "Player2_Ammo")
          (Development|PrintString "bullet")
          (bind _outactors_2 (Actor|GetAllActorsOfClass "/Game/Player2/BP_Player2.BP_Player2_C"))
          (CallFunction|Player2Damage (Variables|/Game/Player2/BP_Player2.BP_Player2_C|GetdamageDelt (Utilities|Array|Get(acopy) _outactors_2)) (Utilities|Array|Get(acopy) _outactors_2))
          (else
            (Development|PrintString "no")))))))

(fn ConstructionScript)