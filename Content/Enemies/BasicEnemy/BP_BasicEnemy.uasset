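; BP_BasicEnemy is a basic enemy character that constantly moves along its arrow's forward direction and fires projectiles.
; BeginPlay caches the player as Enemy, overrides the construction script's Health and AddScore, and starts a looping Fire timer.
; Fire raises IsAttacking, waits briefly, spawns a projectile at the arrow's transform, then clears the flag.
; Look-at-player rotation and attack sound nodes are present but disconnected.
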(event Custom|Fire
  ;[1 1 1] Fire
  (Variables|Default|SetisAttacking true)
  (Utilities|FlowControl|Delay 1.0)
  (Game|SpawnActorfromClass "/Game/Enemies/BasicEnemy/Basic_Enemy_Projectile.Basic_Enemy_Projectile_C" (Transformation|GetWorldTransform (Variables|Default|GetArrow1)) "Undefined" 0 0)
  (Variables|Default|SetisAttacking false))

(event Custom|GetEnemy
  ;[1 1 1] Get Enemy
  (bind _asplayer_character (Utilities|Casting|CastToPlayerCharacter (Game|GetPlayerCharacter 0)))
  (Variables|Default|SetEnemy _asplayer_character))

(event EventBeginPlay
  ;[1 1 1] Begin Play
  (Utilities|FlowControl|Sequence
    (:then_0
      (CallFunction|GetEnemy))
    (:then_1
      (Variables|Default|SetaddScore 5)
      (Variables|Default|SetHealth 25.0))
    (:then_2
      (Utilities|Time|SetTimerbyFunctionName 0 "Fire" (Variables|Default|GetFireRate) true))))

(event EventTick
  (params (DeltaSeconds :type Float%20%28single-precision%29))
  ;[1 1 1] Forward Movement
  (Pawn|Input|AddMovementInput (Math|Vector|GetForwardVector (Variables|Default|GetArrow1)) (Variables|Default|GetSpeed) false))

(fn ConstructionScript
  (|CallParentFunction)
  (Variables|Default|SetHealth 2e+01)
  (Variables|Default|SetaddScore 10))