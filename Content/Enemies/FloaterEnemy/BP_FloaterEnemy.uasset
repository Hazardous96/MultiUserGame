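; Floater enemy that snaps onto one of four cone components on the player when within range, then destroys itself after a delay.
; Looping timers refresh the player reference and check distance, with a DoOnce gating the attach.
; Slots rotate by writing SwitchInt and availability flags to every floater instance; with all four flags false, it destroys itself instead.
; The overlap event is empty, with its destroy logic left disconnected.
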(event OnComponentBeginOverlap(Box)
  (params (OverlappedComponent :type Primitive%20Component%20Object%20Reference) (OtherActor :type Actor%20Object%20Reference) (OtherComp :type Primitive%20Component%20Object%20Reference) (OtherBodyIndex :type Integer) (bFromSweep :type Boolean) (SweepResult :type Hit%20Result%20Structure%20%28by%20ref%29))
  ;[1 1 1] DestroyWhenCollided.
)

(event Custom|Attach%20to%20player
  ;[1 1 1] BeginPlay
  ;;[1 1 1] AttachToPlayer
  (Utilities|IsValid (Variables|Default|GetmyEnemy)
    (:Is%20Valid
      (Variables|Default|Setdistance (Transformation|GetDistanceTo self (Game|GetPlayerCharacter 0)))
      (if (<= (Variables|Default|Getdistance) 5e+03)
        (Utilities|FlowControl|DoOnce false
          (:Completed
            (if (Math|Boolean|ANDBoolean (not (Variables|Default|Getcone1)) (not (Variables|Default|Getcone2)) (not (Variables|Default|Getcone3)) (not (Variables|Default|Getcone4)))
              (Actor|DestroyActor)
              (else
                (switch int (Variables|Default|GetswitchInt)
                  (:0
                    (Transformation|AttachComponentToComponent (Variables|Default|GetCapsuleComponent) (Variables|/Game/PlayerCharacter/PlayerCharacter.PlayerCharacter_C|GetCone (Variables|Default|GetmyEnemy)) "None" "SnapToTarget" "SnapToTarget" "SnapToTarget" true)
                    (bind _outactors (Actor|GetAllActorsOfClass "BP_FloaterEnemy_C"))
                    (for _array_element _outactors
                      (Variables|BP_FloaterEnemy_C|Setcone1 _array_element false)
                      (Variables|BP_FloaterEnemy_C|SetswitchInt _array_element 1))
                    (Utilities|FlowControl|Delay 1e+01)
                    (Actor|DestroyActor)
                    (bind _outactors_2 (Actor|GetAllActorsOfClass "BP_FloaterEnemy_C"))
                    (for _array_element_2 _outactors_2
                      (Variables|BP_FloaterEnemy_C|Setcone1 _array_element_2 true)))
                  (:1
                    (Transformation|AttachComponentToComponent (Variables|Default|GetCapsuleComponent) (Variables|/Game/PlayerCharacter/PlayerCharacter.PlayerCharacter_C|GetCone1 (Variables|Default|GetmyEnemy)) "None" "SnapToTarget" "SnapToTarget" "SnapToTarget" true)
                    (bind _outactors_3 (Actor|GetAllActorsOfClass "BP_FloaterEnemy_C"))
                    (for _array_element_3 _outactors_3
                      (Variables|BP_FloaterEnemy_C|Setcone2 _array_element_3 false)
                      (Variables|BP_FloaterEnemy_C|SetswitchInt _array_element_3 2))
                    (Utilities|FlowControl|Delay 1e+01)
                    (Actor|DestroyActor)
                    (bind _outactors_4 (Actor|GetAllActorsOfClass "BP_FloaterEnemy_C"))
                    (for _array_element_4 _outactors_4
                      (Variables|BP_FloaterEnemy_C|Setcone2 _array_element_4 true)))
                  (:2
                    (Transformation|AttachComponentToComponent (Variables|Default|GetCapsuleComponent) (Variables|/Game/PlayerCharacter/PlayerCharacter.PlayerCharacter_C|GetCone2 (Variables|Default|GetmyEnemy)) "None" "SnapToTarget" "SnapToTarget" "SnapToTarget" true)
                    (bind _outactors_5 (Actor|GetAllActorsOfClass "BP_FloaterEnemy_C"))
                    (for _array_element_5 _outactors_5
                      (Variables|BP_FloaterEnemy_C|Setcone3 _array_element_5 false)
                      (Variables|BP_FloaterEnemy_C|SetswitchInt _array_element_5 3))
                    (Utilities|FlowControl|Delay 1e+01)
                    (Actor|DestroyActor)
                    (bind _outactors_6 (Actor|GetAllActorsOfClass "BP_FloaterEnemy_C"))
                    (for _array_element_6 _outactors_6
                      (Variables|BP_FloaterEnemy_C|Setcone3 _array_element_6 true)))
                  (:3
                    (Transformation|AttachComponentToComponent (Variables|Default|GetCapsuleComponent) (Variables|/Game/PlayerCharacter/PlayerCharacter.PlayerCharacter_C|GetCone3 (Variables|Default|GetmyEnemy)) "None" "SnapToTarget" "SnapToTarget" "SnapToTarget" true)
                    (bind _outactors_7 (Actor|GetAllActorsOfClass "BP_FloaterEnemy_C"))
                    (for _array_element_7 _outactors_7
                      (Variables|BP_FloaterEnemy_C|Setcone4 _array_element_7 false)
                      (Variables|BP_FloaterEnemy_C|SetswitchInt _array_element_7 0))
                    (Utilities|FlowControl|Delay 1e+01)
                    (Actor|DestroyActor)
                    (bind _outactors_8 (Actor|GetAllActorsOfClass "BP_FloaterEnemy_C"))
                    (for _array_element_8 _outactors_8
                      (Variables|BP_FloaterEnemy_C|Setcone4 _array_element_8 true))))))))))))

(event Custom|GetEnemy
  ;[1 1 1] Get Enemy
  (Utilities|IsValid (Variables|Default|GetmyEnemy)
    (:Is%20Not%20Valid
      (bind _asplayer_character (Utilities|Casting|CastToPlayerCharacter (Game|GetPlayerCharacter 0)))
      (Variables|Default|SetmyEnemy _asplayer_character))))

(event EventBeginPlay
  ;[1 1 1] BeginPlay
  (Utilities|Time|SetTimerbyEvent (delegate Custom|Attach%20to%20player) 0.5 true)
  (bind _asplayer_character (Utilities|Casting|CastToPlayerCharacter (Game|GetPlayerCharacter 0)))
  (Variables|Default|SetmyEnemy _asplayer_character)
  (Utilities|Time|SetTimerbyFunctionName 0 "GetEnemy" 0.5 true))

(fn ConstructionScript
  (|CallParentFunction))