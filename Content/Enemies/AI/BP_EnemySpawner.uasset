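; BP_EnemySpawner is an actor that spawns an enemy of the SpawnedEnemy class at its SpawnLocation component after a delay.
; BeginPlay calls StartSpawning, which sets a non-looping SpawnRate timer while EnemiesSpawned is below EnemyCount, otherwise a zero-time one.
; The timer fires SpawnEnemies, which rechecks the count, spawns and increments it.
; Nothing here re-arms the timer, so each StartSpawning call yields at most one enemy.
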(event Custom|StartSpawning
  (if (< (Variables|Default|GetenemiesSpawned) (Variables|Default|GetenemyCount))
    (Utilities|Time|SetTimerbyEvent (delegate Custom|SpawnEnemies) (Variables|Default|GetspawnRate))
    (else
      (Utilities|Time|SetTimerbyEvent (delegate Custom|SpawnEnemies) 0.0))))

(event Custom|SpawnEnemies
  (if true
    (if (< (Variables|Default|GetenemiesSpawned) (Variables|Default|GetenemyCount))
      (Game|SpawnActorfromClass (Variables|Default|GetspawnedEnemy) (Transformation|GetWorldTransform (Variables|Default|GetSpawnLocation)) "Undefined" 0 0)
      (Math|Integer|IncrementInt (Variables|Default|GetenemiesSpawned)))))

(event EventBeginPlay
  (CallFunction|StartSpawning))

(event Collision|EventActorBeginOverlap
  (params (OtherActor :type Actor%20Object%20Reference)))

(event EventTick
  (params (DeltaSeconds :type Float%20%28single-precision%29)))

(fn ConstructionScript)