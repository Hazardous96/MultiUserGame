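; AI controller for BP_Enemy that runs Enemy1BehaviorTree once it possesses an enemy pawn.
; Possession caches the cast pawn, and starts the tree only if that cast succeeds.
; Every tick it writes the player's location, whether the player is within a fixed range, and a "Forward" point to the blackboard.
; That Forward point is a fixed world +X offset from the enemy's location, independent of its rotation.
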(event EventBeginPlay)

(event EventTick
  (params (DeltaSeconds :type Float%20%28single-precision%29))
  (bind _returnvalue (Game|GetPlayerCharacter 0))
  (bind _returnvalue_2 (AI|GetBlackboard 0))
  (AI|Components|Blackboard|SetValueasVector _returnvalue_2 (Utilities|Name|MakeLiteralName "Forward") (+ (Transformation|GetActorLocation (stale EventPossess _asbp_enemy)) "100.000000, 0,0.000000"))
  (AI|Components|Blackboard|SetValueasBool _returnvalue_2 (Utilities|Name|MakeLiteralName "inRange") (<= (Transformation|GetDistanceTo (stale EventPossess _asbp_enemy) _returnvalue) 1e+03))
  (AI|Components|Blackboard|SetValueasVector _returnvalue_2 (Utilities|Name|MakeLiteralName "PlayerLocationKey") (Transformation|GetActorLocation _returnvalue)))

(event EventPossess
  (params (PossessedPawn :type Pawn%20Object%20Reference))
  (bind _asbp_enemy (Utilities|Casting|CastToBP_Enemy PossessedPawn))
  (AI|RunBehaviorTree "/Game/Enemies/AI/Enemy1BehaviorTree.Enemy1BehaviorTree"))

(fn ConstructionScript)