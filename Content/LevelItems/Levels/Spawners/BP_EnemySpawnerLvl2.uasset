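; Enemy spawner that rides far ahead of the player on X and spawns random enemy waves on a looping timer.
; BeginPlay picks the Level 1 or 2 pool, and each tick updates the X position through an SRV wrapper.
; Each wave fills random, non-repeating spawn points from that pool and a separate ground pool, using bool arrays mapped to points.
; The dedicated floater spawn logic is disconnected.
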(event Custom|SRV_SpawnEnemies
  ;[1 1 1] SRV Functions
  (CallFunction|SpawnEnemies)
  (CallFunction|SpawnGroundEnemies))

(event Custom|SpawnEnemies
  ;[1 1 1] SpawnEnemies
  (bind _spawnpositions (CallFunction|AmountandWhere))
  (bind _actors (CallFunction|ConvertBooltoActors _spawnpositions))
  (for _array_element _actors
    (Game|SpawnActorfromClass (.OutItem (Utilities|Array|Random (Variables|Private|GetEnemiesPool))) (Math|Transform|MakeTransform (.location (Transformation|GetWorldTransform _array_element)) (.rotation (Transformation|GetWorldTransform _array_element)) "1,1,1") "Undefined" 0 0)))

(event Custom|SRV_UpdateAttachment
  ;[1 1 1] SRV Functions
  (CallFunction|UpdateAttachment))

(event Custom|UpdateAttachment
  (bind _returnvalue (Transformation|GetActorTransform))
  (bind _returnvalue_2 (Actor|GetActorOfClass "/Game/PlayerCharacter/PlayerCharacter.PlayerCharacter_C"))
  (Utilities|IsValid _returnvalue_2
    (:Is%20Valid
      (Transformation|SetActorTransform (Math|Transform|MakeTransform (Math|Vector|MakeVector (+ (.x (.Location (Math|Transform|BreakTransform (Transformation|GetActorTransform _returnvalue_2)))) 6e+04) (.y (.location _returnvalue)) (.z (.location _returnvalue))) (.rotation _returnvalue) (.scale _returnvalue))))))

(event Custom|SpawnTopFloaters
  ;[1 1 1] SpawnEnemies
)

(event Custom|SpawnGroundEnemies
  ;[1 1 1] SpawnEnemies
  (bind _spawnpositions (CallFunction|Amnt&WhrGround))
  (bind _acotrs (CallFunction|ConvertBooltoActorsGround _spawnpositions))
  (for _array_element _acotrs
    (Game|SpawnActorfromClass (.OutItem (Utilities|Array|Random (Variables|Default|GetGroundEnemies))) (Math|Transform|MakeTransform (.location (Transformation|GetWorldTransform _array_element)) (.rotation (Transformation|GetWorldTransform _array_element)) "1,1,1") "AlwaysSpawn" 0 0)))

(event EventBeginPlay
  ;[1 1 1] Begin Play / Determines Pool
  (if (Variables|Public|GetLevel1)
    (Variables|Private|SetEnemiesPool (Variables|Private|GetLevel1Enemies))
    (else
      (Variables|Private|SetEnemiesPool (Variables|Private|GetLevel2Enemies))))
  (Utilities|Time|SetTimerbyFunctionName 0 "SRV_SpawnEnemies" (Variables|Public|GetSpawnRate) true))

(event EventTick
  (params (DeltaSeconds :type Float%20%28single-precision%29))
  (CallFunction|SRVUpdateAttachment))

(fn ConstructionScript)

(fn AmountandWhere
  ;[1 1 1] Sets A Random Amount of Enemies to spawn (1 on each spawn point at most)
  (bind _output_get (Variables|Private|SetSpawnAmount (Math|Random|RandomIntegerinRange 1 5)))
  (for _index (range 0 _output_get)
    (bind _output_get_2 (LocalVariables|SetCurrentSpot (Math|Random|RandomIntegerinRange 0 (Math|Random|RandomIntegerinRange 1 3))))
    (if (not (Utilities|Array|ContainsItem (LocalVariables|GetTakenSpotsInt) _output_get_2))
      (Utilities|Array|Add (LocalVariables|GetTakenSpotsInt) (LocalVariables|GetCurrentSpot))
      (Utilities|Array|SetArrayElem (LocalVariables|GetTakenSpots) (LocalVariables|GetCurrentSpot) true)))
  (return (LocalVariables|GetTakenSpots)))

(fn ConvertBooltoActors
  (params (Spawn%20Positions :type Array%20of%20Booleans))
  ;[1 1 1] Converts the Bool Positions to actor the Spawn points
  (for (_array_element _array_index) Spawn%20Positions
    (if (Math|Boolean|Equal(Boolean) _array_element true)
      (Utilities|Array|Add (LocalVariables|GetLocations) (Utilities|Array|Get(acopy) (Utilities|Array|MakeArray (Variables|Default|GetFloaterSpawn2) (Variables|Default|GetFloaterSpawn3) (Variables|Default|GetFloaterSpawn4) (Variables|Default|GetFloaterSpawn1) (Variables|Default|GetSpawn6)) _array_index))))
  (return (LocalVariables|GetLocations)))

(fn Amnt&WhrFloatSpwn
  (bind _output_get (Variables|Private|SetFloaterSpawnAmount (Math|Random|RandomIntegerinRange 1 4)))
  (for _index (range 0 _output_get)
    (bind _output_get_2 (LocalVariables|SetCurrentSpot (Math|Random|RandomIntegerinRange 0 (Math|Random|RandomIntegerinRange 2 5))))
    (if (not (Utilities|Array|ContainsItem (LocalVariables|GetTakenSpotsInt) _output_get_2))
      (Utilities|Array|Add (LocalVariables|GetTakenSpotsInt) (LocalVariables|GetCurrentSpot))
      (Utilities|Array|SetArrayElem (LocalVariables|GettakeSpots) (LocalVariables|GetCurrentSpot) true)))
  (return (LocalVariables|GettakeSpots)))

(fn ConvertBooltoActorsFloaters
  (params (Spawn%20Positions :type Array%20of%20Booleans))
  (for (_array_element _array_index) Spawn%20Positions
    (if (Math|Boolean|Equal(Boolean) _array_element true)
      (Utilities|Array|Add (LocalVariables|GetLocations) (Utilities|Array|Get(acopy) (Utilities|Array|MakeArray (Variables|Default|GetFloaterSpawn2) (Variables|Default|GetFloaterSpawn3) (Variables|Default|GetFloaterSpawn4) (Variables|Default|GetFloaterSpawn1)) _array_index))))
  (return (LocalVariables|GetLocations)))

(fn Amnt&WhrGround
  (bind _output_get (Variables|Private|SetSpawnAmount (Math|Random|RandomIntegerinRange 1 3)))
  (for _index (range 0 _output_get)
    (bind _output_get_2 (Variables|Default|SetCurrentSpot (Math|Random|RandomIntegerinRange 0 (Math|Random|RandomIntegerinRange 1 3))))
    (if (not (Utilities|Array|ContainsItem (LocalVariables|GetTakenSpotsInt) _output_get_2))
      (Utilities|Array|Add (LocalVariables|GetTakenSpotsInt) (Variables|Default|GetCurrentSpot))
      (Utilities|Array|SetArrayElem (LocalVariables|GetTakenSpots) (Variables|Default|GetCurrentSpot) true)))
  (return (LocalVariables|GetTakenSpots)))

(fn ConvertBooltoActorsGround
  (params (Spawn%20Positions :type Array%20of%20Booleans))
  (for (_array_element _array_index) Spawn%20Positions
    (if (Math|Boolean|Equal(Boolean) _array_element true)
      (Utilities|Array|Add (LocalVariables|GetLocations) (Utilities|Array|Get(acopy) (Utilities|Array|MakeArray (Variables|StaticComponents|GetSpawn1) (Variables|StaticComponents|GetSpawn3) (Variables|Default|GetSpawn4) (Variables|Default|GetSpawn5)) _array_index))))
  (return (LocalVariables|GetLocations)))