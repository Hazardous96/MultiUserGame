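; Self-chaining track piece for Level 2 that spawns the next piece when a player reaches its trigger and destroys itself once two players have passed.
; On BeginPlay the server randomizes cosmetic meshes and spawns an obstacle at one of two points.
; While BP_Boss1 exists, obstacles are skipped and new pieces get an alternate track.
; A looping timer returns it to the inherited start location when no player character exists, and hits damage players.
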(event OnComponentBeginOverlap(SpawnCollision)
  (params (OverlappedComponent :type Primitive%20Component%20Object%20Reference) (OtherActor :type Actor%20Object%20Reference) (OtherComp :type Primitive%20Component%20Object%20Reference) (OtherBodyIndex :type Integer) (bFromSweep :type Boolean) (SweepResult :type Hit%20Result%20Structure%20%28by%20ref%29))
  ;[1 1 1] Spawns and Deletes Next Chunk
  (if (Actor|ActorHasTag OtherActor "Player")
    (Utilities|FlowControl|DoOnce false
      (:Completed
        (CallFunction|SRVSpawnNextPiece)))))

(event OnComponentBeginOverlap(DestryCollision)
  (params (OverlappedComponent :type Primitive%20Component%20Object%20Reference) (OtherActor :type Actor%20Object%20Reference) (OtherComp :type Primitive%20Component%20Object%20Reference) (OtherBodyIndex :type Integer) (bFromSweep :type Boolean) (SweepResult :type Hit%20Result%20Structure%20%28by%20ref%29))
  ;[1 1 1] Spawns and Deletes Next Chunk
  (if (Actor|ActorHasTag OtherActor "Player")
    (CallFunction|SRVUpdatePassed OtherActor)
    (if (Variables|Private|GetPlayersPassed)
      (Utilities|FlowControl|DoOnce false
        (:Completed
          (CallFunction|SRVDestroyPrevPiece))))))

(event Custom|SRV_SpawnNextPiece
  (bind _spawnpoint (Variables|Default|GetSpawnPoint))
  (bind _spawncollision (Variables|Default|GetSpawnCollision))
  (bind _returnvalue (Transformation|GetWorldTransform _spawnpoint))
  ;[1 1 1] Spawns a new track so this gets overidden
  (Utilities|FlowControl|DoOnce false
    (:Completed
      (bind _returnvalue_2 (Game|SpawnActorfromClass "BP_LevelGenerator2_C" (Math|Transform|MakeTransform (Math|Vector|MakeVector (.x (.location _returnvalue)) (.y (.location _returnvalue)) (.z (.location _returnvalue))) (.rotation _returnvalue) (.scale _returnvalue)) "AlwaysSpawn" 0 0))
      (CallFunction|SetNewTrack _returnvalue_2)
      ;[1 1 1] Skip Over the new begin play
      (Utilities|FlowControl|Delay 1.0)
      (Variables|BP_LevelGenerator2_C|SetStartLocation _returnvalue_2 (Variables|Default|GetStartLocation))
      (Variables|BP_LevelGenerator2_C|SetDialogueNumber _returnvalue_2 (Variables|Default|GetDialogueNumber))
      (if (Utilities|IsValid _spawncollision)
        (Components|DestroyComponent _spawncollision)))))

(event Custom|DestroyPrevPiece
  ;[1 1 1] Destroy Prev Piece
  (Utilities|IsValid self
    (:Is%20Valid
      (Actor|DestroyActor))))

(event Custom|SRV_DestroyPrevPiece
  ;[1 1 1] Destroy Prev Piece
  (CallFunction|DestroyPrevPiece))

(event Custom|SRV_SetEnviroment
  (CallFunction|SetEnviroment))

(event Custom|SRV_CheckDeath
  ;[1 1 1] Checks for player death
  (bind _outactors (Actor|GetAllActorsOfClass "/Game/PlayerCharacter/PlayerCharacter.PlayerCharacter_C"))
  (Utilities|IsValid (Utilities|Array|Get(acopy) _outactors)
    (:Is%20Not%20Valid
      (Transformation|SetActorLocation (Variables|Default|GetStartLocation) false true))))

(event Custom|SRV_SpawnObstacles
  (CallFunction|SetObstacles))

(event Custom|SRV_UpdatePassed
  (params (CurrentCharacter :type Actor%20Object%20Reference))
  (CallFunction|UpdatePassed2 CurrentCharacter))

(event EventBeginPlay
  ;[1 1 1] Checks for player death
  (Variables|Default|SetStartLocation (Transformation|GetActorLocation))
  (Utilities|Time|SetTimerbyEvent (delegate Custom|SRV_CheckDeath) 0.2 true)
  (Networking|SwitchHasAuthority
    (:Authority
      (CallFunction|SRVSetEnviroment)
      (CallFunction|SRVSpawnObstacles))))

(event Collision|EventHit
  (params (MyComp :type Primitive%20Component%20Object%20Reference) (Other :type Actor%20Object%20Reference) (OtherComp :type Primitive%20Component%20Object%20Reference) (bSelfMoved :type Boolean) (HitLocation :type Vector :default "0, 0, 0") (HitNormal :type Vector :default "0, 0, 0") (NormalImpulse :type Vector :default "0, 0, 0") (Hit :type Hit%20Result%20Structure%20%28by%20ref%29))
  ;[1 1 1] Hit
  (if (Actor|ActorHasTag Other "Player")
    (Game|Damage|ApplyDamage Other 5.0 0 0)))

(fn ConstructionScript)

(fn UpdateDialogueNumber
  (bind _result (Utilities|UpdateDialogue)
    (:Exit
      (bind _outactors (Actor|GetAllActorsOfClass "BP_LevelGenerator2_C"))
      (for _array_element _outactors
        (bind _output_get (Variables|BP_LevelGenerator2_C|SetDialogueNumber _array_element _result))
        (return _output_get)))))

(fn DistanceWarning)

(fn SetNewTrack
  (params (NewPiece :type BP%20Level%20Generator%202%20Object%20Reference))
  (bind _track (Variables|BP_LevelGenerator2_C|GetTrack NewPiece))
  (bind _returnvalue (Actor|GetActorOfClass "/Game/Bosses/Boss1/BP_Boss1.BP_Boss1_C"))
  (Utilities|IsValid _returnvalue
    (:Is%20Valid
      (Components|StaticMesh|SetStaticMesh _track (Variables|Defaults|GetTrack1))
      (Transformation|SetRelativeTransform _track (Variables|Defaults|GetTrackOneTransform) false false))))

(fn SetEnviroment
  ;[1 1 1] Set all the cosmetic meshes
  (Utilities|FlowControl|Sequence
    (:then_0
      (for _array_element (Utilities|Array|MakeArray (Variables|Default|GetCosmetic2) (Variables|Default|GetCosmetic3) (Variables|Default|GetCosmetic4) (Variables|Default|GetCosmetic6) (Variables|Default|GetCosmetic7) (Variables|Default|GetCosmetic8))
        (Components|StaticMesh|SetStaticMesh _array_element (Utilities|Array|Get(acopy) (Variables|Private|GetSM_EnviromentPieces) (Math|Random|RandomIntegerinRange 0 (Utilities|Array|Length (Variables|Private|GetSM_EnviromentPieces)))))))
    (:then_1
      (for _array_element_2 (Utilities|Array|MakeArray (Variables|Default|GetCosmetic5) (Variables|Default|GetCosmetic1))
        (Class|SkinnedMeshComponent|SetSkeletalMesh _array_element_2 (Utilities|Array|Get(acopy) (Variables|Private|GetSK_EnviromentPieces) (Math|Random|RandomIntegerinRange 0 (Utilities|Array|Length (Variables|Private|GetSK_EnviromentPieces)))) true)))))

(fn SetObstacles
  (bind _obstacles (Variables|Private|GetObstacles))
  (bind _returnvalue (Utilities|Array|Length _obstacles))
  (bind _returnvalue_2 (Math|Random|RandomIntegerinRange 0 _returnvalue))
  (bind _output (Utilities|Array|Get(acopy) _obstacles _returnvalue_2))
  (bind _returnvalue_3 (Actor|GetActorOfClass "/Game/Bosses/Boss1/BP_Boss1.BP_Boss1_C"))
  (Utilities|IsValid _returnvalue_3
    (:Is%20Not%20Valid
      (if (>= (Math|Random|RandomIntegerinRange 0 100) 50)
        (Game|SpawnActorfromClass _output (Math|Transform|MakeTransform (.location (Transformation|GetWorldTransform (Variables|Default|GetObstacleSpawn%202))) "0, 0, 0" "10.000000,10.000000,10.000000") "Undefined" 0 0)
        (else
          (Game|SpawnActorfromClass _output (Math|Transform|MakeTransform (.location (Transformation|GetWorldTransform (Variables|Default|GetObstacleSpawn1))) "0, 0, 0" "10.000000,10.000000,10.000000") "Undefined" 0 0))))))

(fn UpdatePassed2
  (params (CurrentCharacter :type Actor%20Object%20Reference))
  ;[1 1 1] Checks if Both Players are past
  (Utilities|FlowControl|Sequence
    (:then_0
      (Utilities|IsValid (Variables|Private|Get1stPlayer)
        (:Is%20Valid
          (if (!= (Variables|Private|Get1stPlayer) CurrentCharacter)
            (Variables|Private|Set2ndPlayer CurrentCharacter)))
        (:Is%20Not%20Valid
          (Variables|Private|Set1stPlayer CurrentCharacter))))
    (:then_1
      (Utilities|IsValid (Variables|Private|Get1stPlayer)
        (:Is%20Valid
          (Utilities|IsValid (Variables|Private|Get2ndPlayer)
            (:Is%20Valid
              (Variables|Private|SetPlayersPassed true))))))))