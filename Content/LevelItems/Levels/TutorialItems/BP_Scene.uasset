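; Tutorial scene actor that displays animated pickup props and sends the player on to Level1.
; On BeginPlay, the PickupsMovement timeline bobs and spins the life, ammo, battery, damage and shield components.
; Each update adds the timeline's float and spin values to every component's current relative transform, so the motion accumulates rather than offsetting from a stored origin.
; When the PlayerCharacter overlaps NextLevelTrigger, it opens Level1.
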(event OnComponentBeginOverlap(NextLevelTrigger)
  (params (OverlappedComponent :type Primitive%20Component%20Object%20Reference) (OtherActor :type Actor%20Object%20Reference) (OtherComp :type Primitive%20Component%20Object%20Reference) (OtherBodyIndex :type Integer) (bFromSweep :type Boolean) (SweepResult :type Hit%20Result%20Structure%20%28by%20ref%29))
  (Utilities|Casting|CastToPlayerCharacter OtherActor)
  (Game|OpenLevel(byObjectReference) "/Game/LevelItems/Levels/Level1.Level1"))

(event EventBeginPlay
  (bind _life (Variables|Default|GetLife))
  (bind _ammo (Variables|Default|GetAmmo))
  (bind _bigbattery (Variables|Default|GetBigBattery))
  (bind _smallbattery (Variables|Default|GetSmallBattery))
  (bind _battery (Variables|Default|Getbattery))
  (bind _damage (Variables|Default|GetDamage))
  (bind _shield (Variables|Default|GetShield))
  (bind _returnvalue (Transformation|GetRelativeTransform _shield))
  (bind _returnvalue_2 (Transformation|GetRelativeTransform _life))
  (bind _returnvalue_3 (Transformation|GetRelativeTransform _ammo))
  (bind _returnvalue_4 (Transformation|GetRelativeTransform _bigbattery))
  (bind _returnvalue_5 (Transformation|GetRelativeTransform _smallbattery))
  (bind _returnvalue_6 (Transformation|GetRelativeTransform _battery))
  (bind _returnvalue_7 (Transformation|GetRelativeTransform _damage))
  (bind (_direction _z_float _z_spin) (Timeline|PickupsMovement PlayFromStart)
    (:Update
      (Variables|Private|SetFloatMovement _z_float)
      (Variables|Private|SetSpin _z_spin)
      (Utilities|FlowControl|Sequence
        (:then_0
          (Transformation|SetRelativeTransform _life (Math|Transform|MakeTransform (Math|Vector|MakeVector (.x (.location _returnvalue_2)) (.y (.location _returnvalue_2)) (+ (.z (.location _returnvalue_2)) (Variables|Private|GetFloatMovement))) (Math|Rotator|MakeRotator (.roll (.rotation _returnvalue_2)) (.pitch (.rotation _returnvalue_2)) (- (.yaw (.rotation _returnvalue_2)) (Variables|Private|GetSpin))) (.scale _returnvalue_2)) false false))
        (:then_1
          (Transformation|SetRelativeTransform _ammo (Math|Transform|MakeTransform (Math|Vector|MakeVector (.x (.location _returnvalue_3)) (.y (.location _returnvalue_3)) (+ (.z (.location _returnvalue_3)) (Variables|Private|GetFloatMovement))) (Math|Rotator|MakeRotator (.roll (.rotation _returnvalue_3)) (.pitch (.rotation _returnvalue_3)) (- (.yaw (.rotation _returnvalue_3)) (Variables|Private|GetSpin))) (.scale _returnvalue_3)) false false))
        (:then_2
          (Transformation|SetRelativeTransform _bigbattery (Math|Transform|MakeTransform (Math|Vector|MakeVector (.x (.location _returnvalue_4)) (.y (.location _returnvalue_4)) (+ (.z (.location _returnvalue_4)) (Variables|Private|GetFloatMovement))) (Math|Rotator|MakeRotator (.roll (.rotation _returnvalue_4)) (.pitch (.rotation _returnvalue_4)) (- (.yaw (.rotation _returnvalue_4)) (Variables|Private|GetSpin))) (.scale _returnvalue_4)) false false))
        (:then_3
          (Transformation|SetRelativeTransform _smallbattery (Math|Transform|MakeTransform (Math|Vector|MakeVector (.x (.location _returnvalue_5)) (.y (.location _returnvalue_5)) (+ (.z (.location _returnvalue_5)) (Variables|Private|GetFloatMovement))) (Math|Rotator|MakeRotator (.roll (.rotation _returnvalue_5)) (.pitch (.rotation _returnvalue_5)) (- (.yaw (.rotation _returnvalue_5)) (Variables|Private|GetSpin))) (.scale _returnvalue_5)) false false))
        (:then_4
          (Transformation|SetRelativeTransform _battery (Math|Transform|MakeTransform (Math|Vector|MakeVector (.x (.location _returnvalue_6)) (.y (.location _returnvalue_6)) (+ (.z (.location _returnvalue_6)) (Variables|Private|GetFloatMovement))) (Math|Rotator|MakeRotator (.roll (.rotation _returnvalue_6)) (.pitch (.rotation _returnvalue_6)) (- (.yaw (.rotation _returnvalue_6)) (Variables|Private|GetSpin))) (.scale _returnvalue_6)) false false))
        (:then_5
          (Transformation|SetRelativeTransform _damage (Math|Transform|MakeTransform (Math|Vector|MakeVector (.x (.location _returnvalue_7)) (.y (.location _returnvalue_7)) (+ (.z (.location _returnvalue_7)) (Variables|Private|GetFloatMovement))) (Math|Rotator|MakeRotator (.roll (.rotation _returnvalue_7)) (.pitch (.rotation _returnvalue_7)) (- (.yaw (.rotation _returnvalue_7)) (Variables|Private|GetSpin))) (.scale _returnvalue_7)) false false))
        (:then_6
          (Transformation|SetRelativeTransform _shield (Math|Transform|MakeTransform (Math|Vector|MakeVector (.x (.location _returnvalue)) (.y (.location _returnvalue)) (+ (.z (.location _returnvalue)) (Variables|Private|GetFloatMovement))) (Math|Rotator|MakeRotator (.roll (.rotation _returnvalue)) (.pitch (.rotation _returnvalue)) (- (.yaw (.rotation _returnvalue)) (Variables|Private|GetSpin))) (.scale _returnvalue)) false false))))))

(fn ConstructionScript)