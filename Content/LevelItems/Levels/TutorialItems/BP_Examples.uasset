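; BP_Examples is a tutorial level trigger that shows an example text panel to the player.
; When a PlayerCharacter first overlaps its Box, it creates a BP_ExampleWidget, fills it with its Text variable and adds it to the viewport.
; It also shows the mouse cursor and stops the BP_Scene actor's RotatingMovement by zeroing its rotation rate.
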(event OnComponentBeginOverlap(Box)
  (params (OverlappedComponent :type Primitive%20Component%20Object%20Reference) (OtherActor :type Actor%20Object%20Reference) (OtherComp :type Primitive%20Component%20Object%20Reference) (OtherBodyIndex :type Integer) (bFromSweep :type Boolean) (SweepResult :type Hit%20Result%20Structure%20%28by%20ref%29))
  (bind _returnvalue (Game|GetPlayerController 0))
  (Utilities|Casting|CastToPlayerCharacter OtherActor)
  (Utilities|FlowControl|DoOnce false
    (:Completed
      (bind _returnvalue_2 (UserInterface|CreateWidget "/Game/LevelItems/Levels/TutorialItems/BP_ExampleWidget.BP_ExampleWidget_C" _returnvalue))
      (Default|UpdateText _returnvalue_2 (Variables|Default|GetText))
      (UserInterface|Viewport|AddtoViewport _returnvalue_2 0)
      (Variables|/Script/Engine.PlayerController|SetbShowMouseCursor _returnvalue true)
      (bind _returnvalue_3 (Actor|GetActorOfClass "/Game/LevelItems/Levels/TutorialItems/BP_Scene.BP_Scene_C"))
      (Variables|/Script/Engine.RotatingMovementComponent|SetRotationRate (Variables|/Game/LevelItems/Levels/TutorialItems/BP_Scene.BP_Scene_C|GetRotatingMovement _returnvalue_3) "0, 0, 0"))))

(fn ConstructionScript)