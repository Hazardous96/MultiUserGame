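; BP_DisplaySpawner is a tutorial level item that cycles through random obstacles at its location, showing one at a time.
; BeginPlay fills a list of eight obstacle classes and starts a looping timer on SpawnObstacle.
; Each tick of the timer destroys the previous obstacle and spawns another on authority only, attaching it to the BP_Scene actor.
; The random index range includes the array length, so it can land out of bounds.
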(event Custom|SRV_SpawnObstacle
  (bind _allobstacles (Variables|Default|GetAllObstacles))
  (bind _defaultsceneroot (Variables|Default|GetDefaultSceneRoot))
  (bind _returnvalue (Transformation|GetWorldTransform _defaultsceneroot))
  (Networking|SwitchHasAuthority
    (:Authority
      (bind _returnvalue_2 (Game|SpawnActorfromClass (Utilities|Array|Get(acopy) _allobstacles (Math|Random|RandomIntegerinRange 0 (Utilities|Array|Length _allobstacles))) (Math|Transform|MakeTransform (.location _returnvalue) "0, 0, 0" (.scale _returnvalue)) "AlwaysSpawn" 0 0))
      (bind _returnvalue_3 (Actor|GetActorOfClass "/Game/LevelItems/Levels/TutorialItems/BP_Scene.BP_Scene_C"))
      (Utilities|IsValid _returnvalue_2
        (:Is%20Valid
          (Transformation|AttachActorToActor _returnvalue_2 _returnvalue_3 "None" "KeepWorld" "KeepRelative" "KeepRelative" true)
          (Variables|Default|SetPrevObstacle _returnvalue_2))))))

(event Custom|SpawnObstacle
  (CallFunction|SRVDestroyPrev)
  (CallFunction|SRVSpawnObstacle))

(event Custom|SRV_DestroyPrev
  (bind _prevobstacle (Variables|Default|GetPrevObstacle))
  (Networking|SwitchHasAuthority
    (:Authority
      (Utilities|IsValid _prevobstacle
        (:Is%20Valid
          (Actor|DestroyActor _prevobstacle))))))

(event EventBeginPlay
  (bind _obstacles (Variables|Default|GetObstacles))
  (Variables|Default|SetAllObstacles (Utilities|Array|MakeArray (.obstacle1 _obstacles) (.obstacle2 _obstacles) (.obstacle3 _obstacles) (.obstacle4 _obstacles) (.obstacle5 _obstacles) (.obstacle6 _obstacles) (.obstacle7 _obstacles) (.obstacle8 _obstacles)))
  (Utilities|Time|SetTimerbyFunctionName 0 "SpawnObstacle" 2.5 true))

(fn ConstructionScript)