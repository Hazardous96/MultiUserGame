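; BP_BackgroundGenerator is a self-chaining background landscape piece that extends the level scenery as the player advances.
; On BeginPlay, each piece randomly picks one of two landscape meshes.
; A player-tagged overlap on the Spawn trigger fires once through an SRV event to spawn another piece at SpawnPoint.
; A similar one-shot overlap on the Destroy trigger directly destroys the current piece.
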(event OnComponentBeginOverlap(Spawn)
  (params (OverlappedComponent :type Primitive%20Component%20Object%20Reference) (OtherActor :type Actor%20Object%20Reference) (OtherComp :type Primitive%20Component%20Object%20Reference) (OtherBodyIndex :type Integer) (bFromSweep :type Boolean) (SweepResult :type Hit%20Result%20Structure%20%28by%20ref%29))
  (if (Actor|ActorHasTag OtherActor "Player")
    (Utilities|FlowControl|DoOnce false
      (:Completed
        (CallFunction|SRVSpawnPiece)))))

(event OnComponentBeginOverlap(Destroy)
  (params (OverlappedComponent :type Primitive%20Component%20Object%20Reference) (OtherActor :type Actor%20Object%20Reference) (OtherComp :type Primitive%20Component%20Object%20Reference) (OtherBodyIndex :type Integer) (bFromSweep :type Boolean) (SweepResult :type Hit%20Result%20Structure%20%28by%20ref%29))
  (if (Actor|ActorHasTag OtherActor "Player")
    (Utilities|FlowControl|DoOnce false
      (:Completed
        (Utilities|IsValid self
          (:Is%20Valid
            (CallFunction|DestroyPiece)))))))

(event Custom|SRV_SpawnPiece
  ;[1 1 1] SRV Functions
  (CallFunction|SpawnPiece))

(event Custom|SRV_DestroyPiece
  ;[1 1 1] SRV Functions
  (CallFunction|DestroyPiece))

(event EventBeginPlay
  (bind _mesh (Variables|Default|GetMesh))
  ;[1 1 1] Set Random Landscape
  (if (Math|Random|RandomBool)
    (Components|StaticMesh|SetStaticMesh _mesh "/Game/LevelItems/Levels/Meshes/Landscape1.Landscape1")
    (else
      (Components|StaticMesh|SetStaticMesh _mesh "/Game/LevelItems/Levels/Meshes/Landscape2.Landscape2"))))

(fn ConstructionScript)

(fn SpawnPiece
  ;[1 1 1] Spawns New Piece with random rotation
  (Game|SpawnActorfromClass "BP_BackgroundGenerator_C" (Math|Transform|MakeTransform (Transformation|GetWorldLocation (Variables|Default|GetSpawnPoint)) (Math|Rotator|MakeRotator 0.0 0.0 0.0) "1,1,1") "Undefined" 0 0))

(fn DestroyPiece
  (Actor|DestroyActor))