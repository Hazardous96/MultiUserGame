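; BP_Bounds is a level boundary box that follows the player along X at a set Y and Z and punishes the actor tagged Player1 for leaving it.
; Exiting the box shows a BP_Warning widget and starts looping timers for damage, which grows ten percent per hit, and a death check.
; Re-entering or dying clears the timers, restores the base damage and removes the warning.
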(event OnComponentEndOverlap(BoundBox)
  (params (OverlappedComponent :type Primitive%20Component%20Object%20Reference) (OtherActor :type Actor%20Object%20Reference) (OtherComp :type Primitive%20Component%20Object%20Reference) (OtherBodyIndex :type Integer))
  ;[1 1 1] Overlaps
  (if (Actor|ActorHasTag OtherActor "Player1")
    (Variables|Default|SetCharacter OtherActor)
    (Utilities|FlowControl|DoOnce false
      (:Completed
        (CallFunction|AddWarning)
        (Utilities|Time|SetTimerbyFunctionName 0 "SRV_Damage" 0.5 true)
        (Utilities|Time|SetTimerbyFunctionName 0 "CheckDeath" 0.01 true)))))

(event OnComponentBeginOverlap(BoundBox)
  (params (OverlappedComponent :type Primitive%20Component%20Object%20Reference) (OtherActor :type Actor%20Object%20Reference) (OtherComp :type Primitive%20Component%20Object%20Reference) (OtherBodyIndex :type Integer) (bFromSweep :type Boolean) (SweepResult :type Hit%20Result%20Structure%20%28by%20ref%29))
  ;[1 1 1] Overlaps
  (if (Actor|ActorHasTag OtherActor "Player1")
    (CallFunction|Reset)
    (Utilities|FlowControl|DoOnce false) ; enters at Reset
  ))

(event Custom|SRV_Damage
  (bind _character (Variables|Default|GetCharacter))
  ;[1 1 1] Server Functions
  (Utilities|IsValid _character
    (:Is%20Valid
      (CallFunction|Damage _character))))

(event Custom|Reset
  ;[1 1 1] Reset Value and Timer
  (Utilities|Time|ClearTimerbyFunctionName 0 "SRV_Damage")
  (Variables|Default|SetDamageAmount 5.0)
  (CallFunction|RemoveWarning)
  (Utilities|Time|ClearTimerbyFunctionName 0 "CheckDeath"))

(event Custom|CheckDeath
  ;[1 1 1] Reset Everything if Character dies
  (bind _asplayer_character (Utilities|Casting|CastToPlayerCharacter (Game|GetPlayerCharacter 0)))
  (Utilities|IsValid _asplayer_character
    (:Is%20Valid
      (if (Variables|/Game/PlayerCharacter/PlayerCharacter.PlayerCharacter_C|GetisDead _asplayer_character)
        (Utilities|FlowControl|DoOnce false
          (:Completed
            (CallFunction|Reset)))))))

(event Custom|RemoveWarning
  ;[1 1 1] Add and Remove Warning
  (bind _foundwidgets (Widget|GetAllWidgetsOfClass "/Game/Hud/Widgets/BP_Warning.BP_Warning_C" true))
  (Utilities|IsValid (Utilities|Array|Get(acopy) _foundwidgets)
    (:Is%20Valid
      (Widget|RemovefromParent (Utilities|Array|Get(acopy) _foundwidgets))
      (Utilities|FlowControl|DoOnce false) ; enters at Reset
    )))

(event Custom|UpdateLocation
  ;[1 1 1] Follow Player 1
  (bind _returnvalue (Actor|GetActorOfClass "/Game/PlayerCharacter/PlayerCharacter.PlayerCharacter_C"))
  (Transformation|SetActorLocation (Math|Vector|MakeVector (.x (Transformation|GetActorLocation _returnvalue)) (Variables|Default|GetY%20Location) (Variables|Default|GetZ%20Location)) false false))

(event Custom|AddWarning
  ;[1 1 1] Add and Remove Warning
  (bind _returnvalue (Actor|GetActorOfClass "/Game/PlayerCharacter/PlayerCharacter.PlayerCharacter_C"))
  (bind _asplayer_controller (Utilities|Casting|CastToPlayerController (Pawn|GetController _returnvalue)))
  (bind _returnvalue_2 (UserInterface|CreateWidget "/Game/Hud/Widgets/BP_Warning.BP_Warning_C" (Game|GetPlayerController (Class|GameplayStatics|GetPlayerControllerID _asplayer_controller))))
  (Utilities|FlowControl|DoOnce false
    (:Completed
      (UserInterface|Viewport|AddtoViewport _returnvalue_2 0))))

(event EventTick
  (params (DeltaSeconds :type Float%20%28single-precision%29))
  (CallFunction|UpdateLocation))

(fn ConstructionScript)

(fn Damage
  (params (Character :type Actor%20Object%20Reference))
  (Utilities|IsValid Character
    (:Is%20Valid
      (bind _output_get (Variables|Default|SetDamageAmount (* (Variables|Default|GetDamageAmount) 1.1)))
      (Game|Damage|ApplyDamage Character _output_get 0 0))))