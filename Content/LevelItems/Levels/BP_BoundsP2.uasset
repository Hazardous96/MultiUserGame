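; BP_BoundsP2 is Player 2's level boundary, attached to Player 1's BP_Bounds on BeginPlay.
; When a "Player2"-tagged actor leaves the box, looping timers apply damage that compounds by 10% per tick and poll BP_Player2 for death.
; Re-entry, or death after a short delay, clears the timers and resets the damage.
; DoOnce gates prevent repeat triggers, and authority switches limit BP_Warning widget handling to remote instances.
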(event OnComponentEndOverlap(BoundBox)
  (params (OverlappedComponent :type Primitive%20Component%20Object%20Reference) (OtherActor :type Actor%20Object%20Reference) (OtherComp :type Primitive%20Component%20Object%20Reference) (OtherBodyIndex :type Integer))
  ;[1 1 1] Overlaps
  (if (Actor|ActorHasTag OtherActor "Player2")
    (Utilities|FlowControl|Sequence
      (:then_0
        (Variables|Default|SetCharacter OtherActor)
        (Utilities|FlowControl|DoOnce false
          (:Completed
            (CallFunction|AddWarning)
            (Utilities|Time|SetTimerbyFunctionName 0 "SRV_Damage" 0.5 true)
            (Utilities|Time|SetTimerbyFunctionName 0 "CheckDeath" 0.01 true))))
      (:then_1
        (Utilities|FlowControl|DoOnce true) ; enters at Reset
      ))))

(event OnComponentBeginOverlap(BoundBox)
  (params (OverlappedComponent :type Primitive%20Component%20Object%20Reference) (OtherActor :type Actor%20Object%20Reference) (OtherComp :type Primitive%20Component%20Object%20Reference) (OtherBodyIndex :type Integer) (bFromSweep :type Boolean) (SweepResult :type Hit%20Result%20Structure%20%28by%20ref%29))
  ;[1 1 1] Overlaps
  (if (Actor|ActorHasTag OtherActor "Player2")
    (Utilities|FlowControl|DoOnce true
      (:Completed
        (CallFunction|Reset)
        (Utilities|FlowControl|DoOnce false) ; enters at Reset
      ))))

(event Custom|SRV_Damage
  (bind _character (Variables|Default|GetCharacter))
  ;[1 1 1] Server Functions
  (Utilities|IsValid _character
    (:Is%20Valid
      (CallFunction|Damage _character))))

(event Custom|Reset
  ;[1 1 1] Reset Value and Timer
  (Utilities|Time|ClearTimerbyFunctionName 0 "SRV_Damage")
  (Variables|Default|SetDamageAmount 5.0)
  (CallFunction|RemoveWarning)
  (Utilities|Time|ClearTimerbyFunctionName 0 "CheckDeath"))

(event Custom|RemoveWarning
  ;[1 1 1] Add and Remove Warning
  (Networking|SwitchHasAuthority
    (:Remote
      (Utilities|FlowControl|Sequence
        (:then_0
          (bind _foundwidgets (Widget|GetAllWidgetsOfClass "/Game/Hud/Widgets/BP_Warning.BP_Warning_C" false))
          (for _array_element _foundwidgets
            (Utilities|IsValid _array_element
              (:Is%20Valid
                (Widget|RemovefromParent _array_element))))
          (Utilities|FlowControl|DoOnce false) ; enters at Reset
        )
        (:then_1
          (Utilities|FlowControl|DoOnce false) ; enters at Reset
        )))))

(event Custom|CheckDeath
  ;[1 1 1] Reset Everything if Character dies
  (bind _returnvalue (Actor|GetActorOfClass "/Game/Player2/BP_Player2.BP_Player2_C"))
  (Utilities|IsValid _returnvalue
    (:Is%20Valid
      (if (Variables|/Game/Player2/BP_Player2.BP_Player2_C|GetisDead _returnvalue)
        (Utilities|FlowControl|DoOnce false
          (:Completed
            (Utilities|FlowControl|Delay 3.0)
            (CallFunction|Reset)))))))

(event Custom|AddWarning
  ;[1 1 1] Add and Remove Warning
  (Networking|SwitchHasAuthority
    (:Remote
      (Utilities|FlowControl|DoOnce false
        (:Completed
          (bind _returnvalue (Actor|GetActorOfClass "/Game/Player2/BP_Player2.BP_Player2_C"))
          (bind _asplayer_controller (Utilities|Casting|CastToPlayerController (Pawn|GetController _returnvalue)))
          (bind _returnvalue_2 (UserInterface|CreateWidget "/Game/Hud/Widgets/BP_Warning.BP_Warning_C" (Game|GetPlayerController (Class|GameplayStatics|GetPlayerControllerID _asplayer_controller))))
          (Utilities|FlowControl|DoOnce false
            (:Completed
              (UserInterface|Viewport|AddtoViewport _returnvalue_2 0))))))))

(event EventBeginPlay
  ;[1 1 1] Attach to Player 1's Bounds
  (bind _returnvalue (Actor|GetActorOfClass "/Game/LevelItems/Levels/BP_Bounds.BP_Bounds_C"))
  (Transformation|AttachActorToActor _returnvalue "None" "SnapToTarget" "KeepWorld" "SnapToTarget" true))

(fn ConstructionScript)

(fn Damage
  (params (Character :type Actor%20Object%20Reference))
  (Utilities|IsValid Character
    (:Is%20Valid
      (bind _output_get (Variables|Default|SetDamageAmount (* (Variables|Default|GetDamageAmount) 1.1)))
      (Game|Damage|ApplyDamage Character _output_get 0 0))))