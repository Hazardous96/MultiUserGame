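; BP_BaseObstacle is a shootable obstacle that damages a Player-tagged actor on hit and then destroys itself.
; On BeginPlay it caches Player1 plus either Player2 or the NPC, depending on the game instance's multiplayer flag.
; Incoming damage uses the causer's ammo tag to award points to the matching shooter, re-fetching references if invalid.
; Tagged shots also reduce Health, destroying the obstacle once it drops below zero.
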(event Custom|getPlayers
  (bind _returnvalue (Actor|GetActorOfClass "/Game/PlayerCharacter/PlayerCharacter.PlayerCharacter_C"))
  (Variables|Default|SetPlayer1 _returnvalue)
  (bind _asonline_game_instance (Utilities|Casting|CastToOnlineGameInstance (Game|GetGameInstance)))
  (if (Variables|/Game/Player2/Multiplayer/OnlineGameInstance.OnlineGameInstance_C|GetIsMultiplayer _asonline_game_instance)
    (bind _returnvalue_2 (Actor|GetActorOfClass "/Game/Player2/BP_Player2.BP_Player2_C"))
    (Variables|Default|SetPlayer2 _returnvalue_2)
    (else
      (bind _returnvalue_3 (Actor|GetActorOfClass "/Game/NPC/BP_NPC.BP_NPC_C"))
      (Variables|Default|SetNPC _returnvalue_3))))

(event EventBeginPlay
  (CallFunction|GetPlayers))

(event Game|Damage|EventAnyDamage
  (params (Damage :type Float%20%28single-precision%29) (DamageType :type Damage%20Type%20Object%20Reference) (InstigatedBy :type Controller%20Object%20Reference) (DamageCauser :type Actor%20Object%20Reference))
  (bind _player1 (Variables|Default|GetPlayer1))
  (bind _npc (Variables|Default|GetNPC))
  (bind _player2 (Variables|Default|GetPlayer2))
  ;[1 1 1] Take damage if shot from player
  (if (Actor|ActorHasTag DamageCauser "Player1_Ammo")
    (Utilities|IsValid _player1
      (:Is%20Valid
        _)
      (:Is%20Not%20Valid
        (CallFunction|GetPlayers)))
    (Variables|/Game/PlayerCharacter/PlayerCharacter.PlayerCharacter_C|SetScore _player1 (+ (Variables|/Game/PlayerCharacter/PlayerCharacter.PlayerCharacter_C|GetScore _player1) 20))
    (Variables|Default|Sethealth (- (Variables|Default|Gethealth) Damage) :!label _label)
    (if (not (>= (Variables|Default|Gethealth) 0.0))
      (Actor|DestroyActor))
    (elif (Actor|ActorHasTag DamageCauser "NPC_Ammo")
      (Utilities|IsValid 0
        (:Is%20Valid
          _)
        (:Is%20Not%20Valid
          (CallFunction|GetPlayers)))
      (Variables|/Game/NPC/BP_NPC.BP_NPC_C|SetScore _npc (+ (Variables|/Game/NPC/BP_NPC.BP_NPC_C|GetScore _npc) 20))
      (goto _label)
      (else
        (Utilities|IsValid _player2
          (:Is%20Valid
            _)
          (:Is%20Not%20Valid
            (CallFunction|GetPlayers)))
        (if (Actor|ActorHasTag DamageCauser "Player2_Ammo")
          (Variables|/Game/Player2/BP_Player2.BP_Player2_C|SetScore _player2 (+ (Variables|/Game/Player2/BP_Player2.BP_Player2_C|GetScore _player2) 20))
          (goto _label))))))

(event Collision|EventHit
  (params (MyComp :type Primitive%20Component%20Object%20Reference) (Other :type Actor%20Object%20Reference) (OtherComp :type Primitive%20Component%20Object%20Reference) (bSelfMoved :type Boolean) (HitLocation :type Vector :default "0, 0, 0") (HitNormal :type Vector :default "0, 0, 0") (NormalImpulse :type Vector :default "0, 0, 0") (Hit :type Hit%20Result%20Structure%20%28by%20ref%29))
  ;[1 1 1] Destroy and apply damage if player hits obstacle
  (Utilities|IsValid Other
    (:Is%20Valid
      (if (Actor|ActorHasTag Other "Player")
        (Game|Damage|ApplyDamage Other (Variables|Default|Getdamage) 0 0)
        (Actor|DestroyActor)))))

(fn ConstructionScript)