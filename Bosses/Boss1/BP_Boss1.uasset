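; First boss actor that attacks the player with laser volleys and a heavy beam until its health runs out.
; A looping action selector randomly favors timer-driven twin shots over the delayed beam.
; Attacks trace toward a point offset from the player and require successful screen projection of the boss; shots add random spread.
; Damage switches phase at half health, where the selector has no attacks, and destroys it at zero.
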(event Custom|RightLaserShot
  (bind _lasershot2 (Variables|Default|GetLaserShot2))
  (bind _returnvalue (Transformation|GetWorldLocation _lasershot2))
  ;[1 1 1] LaserShot
  (bind _outhit (Collision|LineTraceByChannel (Transformation|GetWorldLocation (Variables|Default|GetLaserShot2)) (+ (Transformation|GetWorldLocation (Variables|/Script/Engine.Actor|GetRootComponent (Game|GetPlayerCharacter 0))) "2000.000000, 0, 0") "TraceTypeQuery2" false 0 "None"))
  (if (.ReturnValue (Class|PlayerController|ProjectWorldLocationtoScreen (Game|GetPlayerController 0) (Transformation|GetActorLocation) false))
    (Game|SpawnActorfromClass "/Game/Bosses/Boss1/BP_Boss1LaserShot.BP_Boss1LaserShot_C" (Math|Transform|MakeTransform _returnvalue (Math|Rotator|FindLookatRotation _returnvalue (Math|Random|RandomPointinBoundingBox (Math|Vector|SelectVector (.ImpactPoint (Collision|BreakHitResult _outhit)) (.TraceEnd (Collision|BreakHitResult _outhit)) (.bBlockingHit (Collision|BreakHitResult _outhit))) "0.000000,1000.000000,1000.000000"))) "Undefined" 0 0)))

(event Custom|ActionSelector
  (if (== (Variables|Default|GetPhase) 0) :!label _label
    (switch int (Math|Random|RandomIntegerinRange 0 4)
      (:0
        _)
      (:1
        _)
      (:2
        _)
      (:3
        _)
      (:4
        (CallFunction|LaserBeam)
        (Utilities|FlowControl|Delay 5.0)
        (goto _label)))
    (bind _returnvalue (Utilities|Time|SetTimerbyEvent (delegate Custom|LeftLaserShot) 0.25 true))
    (bind _returnvalue_2 (Utilities|Time|SetTimerbyEvent (delegate Custom|RightLaserShot) 0.25 true))
    (Utilities|FlowControl|Delay 5.0)
    (Utilities|Time|PauseTimerbyHandle _returnvalue)
    (Utilities|Time|PauseTimerbyHandle _returnvalue_2)
    (Utilities|FlowControl|Delay 2.5)
    (goto _label)))

(event Custom|LeftLaserShot
  (bind _lasershot1 (Variables|Default|GetLaserShot1))
  (bind _returnvalue (Transformation|GetWorldLocation _lasershot1))
  ;[1 1 1] LaserShot
  (bind _outhit (Collision|LineTraceByChannel (Transformation|GetWorldLocation (Variables|Default|GetLaserShot1)) (+ (Transformation|GetWorldLocation (Variables|/Script/Engine.Actor|GetRootComponent (Game|GetPlayerCharacter 0))) "2000.000000,0.000000, 0") "TraceTypeQuery2" false 0 "None"))
  (if (.ReturnValue (Class|PlayerController|ProjectWorldLocationtoScreen (Game|GetPlayerController 0) (Transformation|GetActorLocation) false))
    (Game|SpawnActorfromClass "/Game/Bosses/Boss1/BP_Boss1LaserShot.BP_Boss1LaserShot_C" (Math|Transform|MakeTransform _returnvalue (Math|Rotator|FindLookatRotation _returnvalue (Math|Random|RandomPointinBoundingBox (Math|Vector|SelectVector (.ImpactPoint (Collision|BreakHitResult _outhit)) (.TraceEnd (Collision|BreakHitResult _outhit)) (.bBlockingHit (Collision|BreakHitResult _outhit))) "0.000000,1000.000000,1000.000000"))) "Undefined" 0 0)))

(event Custom|LaserBeam
  (bind _bigattack (Variables|Default|GetBigAttack))
  (bind _returnvalue (Transformation|GetWorldLocation _bigattack))
  ;[1 1 1] LaserBeam
  (bind _outhit (Collision|LineTraceByChannel (Transformation|GetWorldLocation (Variables|Default|GetBigAttack)) (+ (Transformation|GetWorldLocation (Variables|/Script/Engine.Actor|GetRootComponent (Game|GetPlayerCharacter 0))) "2000.000000, 0, 0") "TraceTypeQuery2" false 0 "ForDuration"))
  (if (.ReturnValue (Class|PlayerController|ProjectWorldLocationtoScreen (Game|GetPlayerController 0) (Transformation|GetActorLocation) false))
    (Utilities|FlowControl|Delay 1.5)
    (Game|SpawnActorfromClass "/Game/Bosses/Boss1/BP_Boss1LaserBeam.BP_Boss1LaserBeam_C" (Math|Transform|MakeTransform _returnvalue (Math|Rotator|FindLookatRotation _returnvalue (Math|Vector|SelectVector (.ImpactPoint (Collision|BreakHitResult _outhit)) (.TraceEnd (Collision|BreakHitResult _outhit)) (.bBlockingHit (Collision|BreakHitResult _outhit))))) "Undefined" 0 0)))

(event Game|Damage|EventAnyDamage
  (params (Damage :type Float%20%28single-precision%29) (DamageType :type Damage%20Type%20Object%20Reference) (InstigatedBy :type Controller%20Object%20Reference) (DamageCauser :type Actor%20Object%20Reference))
  (bind _output_get (Variables|Default|SetHealth (- (Variables|Default|GetHealth) Damage)))
  (Development|PrintString (Utilities|String|ToString(Float) _output_get))
  (if (<= _output_get (Variables|Default|GetPhase_Change))
    (Variables|Default|SetPhase 1)
    (if (<= (Variables|Default|GetHealth) 0.0)
      (Actor|DestroyActor))
    (else
      (Variables|Default|SetPhase 0))))

(event EventTick
  (params (DeltaSeconds :type Float%20%28single-precision%29))
  (|CallParentFunction DeltaSeconds) ; This node is disabled and will not be called.\nDrag off pins to build functionality.
)

(event EventBeginPlay
  (Variables|Default|SetHealth 3e+02)
  (Variables|Default|SetPhase_Change 1.5e+02)
  (CallFunction|ActionSelector))

(fn ConstructionScript
  (|CallParentFunction))